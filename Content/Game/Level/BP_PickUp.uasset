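; Weapon pickup actor that adds its configured weapon, with minimum bullets from WorldData, to the inventory of an overlapping BP_Player.
; The authority tracks the overlapping player and retries the grant each tick while off cooldown, restarting the timer only when the weapon is added.
; The mesh spins from a random starting yaw and lerps its scale to zero during cooldown, then back.
; Reset restores the initial availability from AvailableOnStart.
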(event OnComponentBeginOverlap(Sphere)
  (params (OverlappedComponent :type Primitive%20Component%20Object%20Reference) (OtherActor :type Actor%20Object%20Reference) (OtherComp :type Primitive%20Component%20Object%20Reference) (OtherBodyIndex :type Integer) (bFromSweep :type Boolean) (SweepResult :type Hit%20Result%20Structure%20%28by%20ref%29))
  (Networking|SwitchHasAuthority
    (:Authority
      (bind _asbp_player (Utilities|Casting|CastToBP_Player OtherActor))
      (Variables|Default|SetTriggeredPlayer _asbp_player))))

(event OnComponentEndOverlap(Sphere)
  (params (OverlappedComponent :type Primitive%20Component%20Object%20Reference) (OtherActor :type Actor%20Object%20Reference) (OtherComp :type Primitive%20Component%20Object%20Reference) (OtherBodyIndex :type Integer))
  (Networking|SwitchHasAuthority
    (:Authority
      (if (== OtherActor (Variables|Default|GetTriggeredPlayer))
        (Variables|Default|SetTriggeredPlayer 0)))))

(event Custom|AddBonusLocalRPC
  (params (Player :type BP%20Player%20Object%20Reference))
  (CallFunction|AddBonus Player))

(event EventBeginPlay
  (Transformation|AddLocalRotation (Variables|Default|GetScene) (Math|Rotator|MakeRotator 0.0 0.0 (Math|Random|RandomFloatinRange 0.0 3.6e+02)) false false)
  (Variables|Default|SetStartScale (Variables|/Script/Engine.SceneComponent|GetRelativeScale3D (Variables|Default|GetSkeletalMesh)))
  (for _index (range 0 (Rendering|Material|GetNumMaterials (Variables|Default|GetSkeletalMesh)))
    (Rendering|Material|SetMaterial (Variables|Default|GetSkeletalMesh) _index (Variables|Default|GetMaterial))
    (for _index_2 (range 0 (Rendering|Material|GetNumMaterials (Variables|Default|GetSphere1)))
      (Rendering|Material|SetMaterial (Variables|Default|GetSphere1) _index_2 (Variables|Default|GetMaterial)))))

(event EventTick
  (params (DeltaSeconds :type Float%20%28single-precision%29))
  (bind _triggeredplayer (Variables|Default|GetTriggeredPlayer))
  (CallFunction|Rotation DeltaSeconds)
  (CallFunction|VisibilityUpdate DeltaSeconds)
  (Networking|SwitchHasAuthority
    (:Authority
      (CallFunction|CheckAdd DeltaSeconds)
      (if (not (Variables|Default|GetIsCooldown))
        (Utilities|IsValid _triggeredplayer
          (:Is%20Valid
            (CallFunction|AddBonusLocalRPC _triggeredplayer)))))))

(fn ConstructionScript)

(fn AddBonus
  (params (Player :type BP%20Player%20Object%20Reference))
  (Variables|Default|SetTriggeredPlayer Player)
  (Utilities|IsValid Player
    (:Is%20Valid
      (bind _isadded (CallFunction|AddLogic))
      (if _isadded
        (Variables|Default|SetTime 0.0)
        (Variables|Default|SetIsCooldown true)))))

(fn Rotation
  (params (TimeDelta :type Float%20%28double-precision%29))
  (Transformation|AddActorLocalRotation (Math|Rotator|MakeRotator 0.0 0.0 (* 1e+01 TimeDelta (Variables|Default|GetRotateMult))) false false))

(fn VisibilityUpdate
  (params (Delta :type Float%20%28double-precision%29))
  (LocalVariables|SetDeltaTime (* Delta 25.0))
  (if (not (Variables|Default|GetIsCooldown))
    (bind _output_get (LocalVariables|SetTargetVector (Variables|Default|GetStartScale)))
    (Transformation|SetRelativeScale3D (Variables|Default|GetSkeletalMesh) (Math|Vector|Lerp(Vector) (Variables|/Script/Engine.SceneComponent|GetRelativeScale3D (Variables|Default|GetSkeletalMesh)) _output_get (LocalVariables|GetDeltaTime)))
    (else
      (bind _output_get_2 (LocalVariables|SetTargetVector "0, 0, 0"))
      (Transformation|SetRelativeScale3D (Variables|Default|GetSkeletalMesh) (Math|Vector|Lerp(Vector) (Variables|/Script/Engine.SceneComponent|GetRelativeScale3D (Variables|Default|GetSkeletalMesh)) _output_get_2 (LocalVariables|GetDeltaTime))))))

(fn CheckAdd
  (params (Delta :type Float%20%28double-precision%29))
  (if (Variables|Default|GetIsCooldown)
    (Variables|Default|SetTime (+ (Variables|Default|GetTime) Delta))
    (if (>= (Variables|Default|GetTime) (Variables|Default|GetCooldown))
      (Variables|Default|SetIsCooldown false))))

(fn AddLogic
  (bind _isadded (Default|AddWeapon (Variables|/Game/Game/Player/BP_Player.BP_Player_C|GetBP_InventoryComponent (Variables|Default|GetTriggeredPlayer)) (Utilities|Struct|MakeST_Item (Variables|Default|GetWeapon) (Math|Conversions|ToFloat(Integer) (Variables|/Script/ShooterRooms.WeaponDataAsset|GetminBullets (.Value (Utilities|Map|Find (Variables|/Script/ShooterRooms.WorldData|GetweaponsList (Variables|Default|GetWorldData)) (Variables|Default|GetWeapon))))))))
  (return _isadded))

(fn Reset
  (if (Variables|Default|GetAvailableOnStart)
    (Variables|Default|SetIsCooldown false)
    (Variables|Default|SetTime (Variables|Default|GetCooldown))
    (else
      (Variables|Default|SetIsCooldown true)
      (Variables|Default|SetTime 0.0))))