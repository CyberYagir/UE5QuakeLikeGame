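; BP_EndCharacter is an end-game display character that shows a player's number and name over a randomized look and animation.
; On init it hides four skeletal meshes, reveals one at random and plays a random montage from its list on the main skeletal mesh.
; It then passes a "#" label, built from the one-based player Id and the stats name, to its BP_PlayerWinText_UI widget.
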(event Custom|Init
  (params (PlayerStats :type ST%20Player%20Stas%20Structure) (Id :type Integer))
  (CallFunction|OnInit)
  (bind _asbp_player_win_text_ui (Utilities|Casting|CastToBP_PlayerWinText_UI (UserInterface|GetWidget (Variables|Default|GetWidget))))
  (Default|Init _asbp_player_win_text_ui (Utilities|String|StringToName (Utilities|String|Append "#" (Utilities|String|ToString(Integer) (+ Id 1)) " " (Utilities|String|ToString(Name) (.Name (Utilities|Struct|BreakST_PlayerStas PlayerStats)))))))

(event Custom|OnInit
  (bind _skeletalmesh1 (Variables|Default|GetSkeletalMesh1))
  (bind _skeletalmesh2 (Variables|Default|GetSkeletalMesh2))
  (bind _skeletalmesh3 (Variables|Default|GetSkeletalMesh3))
  (bind _skeletalmesh4 (Variables|Default|GetSkeletalMesh4))
  (bind _array (Utilities|Array|MakeArray _skeletalmesh1 _skeletalmesh2 _skeletalmesh3 _skeletalmesh4))
  (for _array_element _array
    (Rendering|SetVisibility _array_element false true))
  (Rendering|SetVisibility (.OutItem (Utilities|Array|Random _array)) true false)
  (Animation|Montage|PlayMontage (Variables|Default|GetSkeletalMesh) (.OutItem (Utilities|Array|Random (Variables|Default|GetMontages)))))

(fn ConstructionScript)