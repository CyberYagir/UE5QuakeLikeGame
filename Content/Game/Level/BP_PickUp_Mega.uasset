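; BP_PickUp_Mega is a level pickup that grants typed points to the triggering player's stats component.
; Its AddLogic adds the full points when buffed; otherwise it checks IsCanAdd and adds only the allowed amount.
; A successful add resets the timer, starts cooldown and returns true, while a refused add returns false.
; The event graph holds only disabled stub events.
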(event EventBeginPlay
  (|CallParentFunction) ; This node is disabled and will not be called.\nDrag off pins to build functionality.
)

(event Collision|EventActorBeginOverlap
  (params (OtherActor :type Actor%20Object%20Reference)))

(event EventTick
  (params (DeltaSeconds :type Float%20%28single-precision%29))
  (|CallParentFunction DeltaSeconds) ; This node is disabled and will not be called.\nDrag off pins to build functionality.
)

(fn ConstructionScript
  (|CallParentFunction))

(fn AddLogic
  (bind _triggeredplayer (Variables|Default|GetTriggeredPlayer))
  (bind _bp_statscomponent (Variables|/Game/Game/Player/BP_Player.BP_Player_C|GetBP_StatsComponent _triggeredplayer))
  (if (Variables|Default|GetIsBuffed)
    (Default|AddPoints (Variables|/Game/Game/Player/BP_Player.BP_Player_C|GetBP_StatsComponent (Variables|Default|GetTriggeredPlayer)) (Variables|Default|GetType) (Variables|Default|GetPoints) (Variables|Default|GetIsBuffed))
    (else
      (bind (_iscan _canaddvalue) (Default|IsCanAdd _bp_statscomponent (Variables|Default|GetIsBuffed) (Variables|Default|GetType) (Variables|Default|GetPoints)))
      (if _iscan
        (Default|AddPoints _bp_statscomponent (Variables|Default|GetType) _canaddvalue (Variables|Default|GetIsBuffed))
        (else
          (return false)))))
  (Variables|Default|SetTime 0.0)
  (Variables|Default|SetIsCooldown true)
  (return true))