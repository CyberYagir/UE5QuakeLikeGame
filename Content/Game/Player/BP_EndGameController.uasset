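; BP_EndGameController pushes its camera forward when play begins, apparently for the end-game screen or sequence.
; On BeginPlay it stores the camera's world location and a target 50 units along its forward vector.
; A timeline's SmoothMove track then drives a lerp between the two points, setting the camera's world location on each update without sweeping.
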(event EventBeginPlay
  (Variables|Default|SetStartPos (Transformation|GetWorldLocation (Variables|Default|GetCamera)))
  (Variables|Default|SetTargetPos (+ (Transformation|GetWorldLocation (Variables|Default|GetCamera)) (* (Math|Vector|GetForwardVector (Variables|Default|GetCamera)) 5e+01)))
  (bind _smoothmove (Timeline|Timeline Play)
    (:Update
      (Transformation|SetWorldLocation (Variables|Default|GetCamera) (Math|Vector|Lerp(Vector) (Variables|Default|GetStartPos) (Variables|Default|GetTargetPos) _smoothmove) false false))))

(fn ConstructionScript)