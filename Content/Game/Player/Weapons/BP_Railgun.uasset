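; BP_Railgun is the player's railgun weapon, which fires a laser shot through the multiplayer handler.
; On shoot, it removes a bullet from the current weapon, activates the LaserFire effect and calls ShootProjectile.
; ShootProjectile projects a distant end point along the camera's forward vector and orients the muzzle transform toward it.
; It passes that transform, both camera points and the weapon's damage to ShootRailServer on the player's BPMultiplayerHandlerComponent.
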(event EventOnShootBullets
  (Default|RemoveBulletfromCurrentWeapon (Variables|Default|GetPlayer) false)
  (Components|Activation|Activate (Variables|Default|GetLaser_Fire) true)
  (CallFunction|ShootProjectile))

(fn ConstructionScript)

(fn ShootProjectile
  (bind _point (Variables|Default|GetPoint))
  (bind _returnvalue (Transformation|GetWorldTransform _point))
  (bind (_location _rotation _scale) (Math|Transform|BreakTransform _returnvalue))
  (LocalVariables|SetCamera (Variables|/Game/Game/Player/BP_Player.BP_Player_C|GetCamera (Variables|Default|GetPlayer)))
  (bind _output_get (LocalVariables|SetEndPos (+ (Transformation|GetWorldLocation (LocalVariables|GetCamera)) (* (Math|Vector|GetForwardVector (LocalVariables|GetCamera)) 100000))))
  (Default|ShootRailServer (Variables|/Game/Game/Player/BP_Player.BP_Player_C|GetBP_MultiplayerHandlerComponent (Variables|Default|GetPlayer)) (Math|Transform|MakeTransform _location (Math|Rotator|FindLookatRotation _location (LocalVariables|GetEndPos)) _scale) _output_get (Transformation|GetWorldLocation (LocalVariables|GetCamera)) (Variables|/Script/ShooterRooms.WeaponDataAsset|Getdamage (Variables|Default|GetWeaponData))))