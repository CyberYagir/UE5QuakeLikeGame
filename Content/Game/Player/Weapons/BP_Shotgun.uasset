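; BP_Shotgun is a player shotgun that fires a double blast per shot.
; On shooting it removes a bullet, fires and triggers a Niagara effect, then fires again after a short delay with a second effect.
; Each blast sends camera transform, pellet count, spread and per-pellet damage (weapon damage divided by burst count) to the player's multiplayer handler component for server-side shooting.
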(event EventOnShootBullets
  (Default|RemoveBulletfromCurrentWeapon (Variables|Default|GetPlayer) false)
  (CallFunction|ShootProjectile)
  (Components|Activation|Activate (Variables|Default|GetNiagara) false)
  (Utilities|FlowControl|Delay 0.2)
  (CallFunction|ShootProjectile)
  (Components|Activation|Activate (Variables|Default|GetNiagara1) false))

(fn ConstructionScript)

(fn ShootProjectile
  (bind _player (Variables|Default|GetPlayer))
  (bind _camera (Variables|/Game/Game/Player/BP_Player.BP_Player_C|GetCamera _player))
  (Default|ShootShotgunServer (Variables|/Game/Game/Player/BP_Player.BP_Player_C|GetBP_MultiplayerHandlerComponent (Variables|Default|GetPlayer)) (Transformation|GetWorldRotation _camera) (Transformation|GetWorldLocation _camera) (Variables|Default|GetBurstCount) (Variables|Default|GetSpreadAngle) (/ (Variables|/Script/ShooterRooms.WeaponDataAsset|Getdamage (Variables|Default|GetWeaponData)) (Variables|Default|GetBurstCount))))