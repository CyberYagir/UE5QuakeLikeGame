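; Continuous laser-beam weapon for the player, with firing blocked until the equip montage completes.
; While firing, the owner's rate-limited Tick spends ammo, traces from the camera, drives the Niagara beam and hit effect, and requests per-tick server damage.
; Beam state and endpoint go through the player's multiplayer handler.
; Non-owners swap to a client laser asset and mirror that data from a weapon socket.
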(event EventBeginPlay
  (Actor|Tick|SetActorTickInterval (/ 1.0 (Math|Conversions|ToFloat(Integer) (Variables|/Script/ShooterRooms.WeaponDataAsset|GettickRate (Variables|Default|GetWeaponData)))))
  (CallFunction|GetPlayer)
  (Variables|Default|SetweaponState "VE_Equip")
  (Variables|Default|SetwaitForEquip true)
  (Animation|Montage|PlayMontage (Variables|Default|GetSkeletalMesh) (Variables|Default|GetEquip_Montage)
    (:OnCompleted
      (Variables|Default|SetwaitForEquip false)
      (Variables|Default|SetweaponState "VE_Idle")
      (Variables|Default|SetStartLaserScale 1.0)
      (Effects|Components|ParticleSystem|SetFloatParameter (Variables|Default|GetShaft_Laser) "Scale" 0.0)
      (if (not (Variables|/Game/Game/Player/BP_Player.BP_Player_C|GetIsMine (Variables|Default|GetPlayer)))
        (Class|NiagaraComponent|SetAsset (Variables|Default|GetShaft_Laser) "/Game/Game/Particles/Shaft_Laser_Client.Shaft_Laser_Client" false)))))

(event EventOnShoot
  (Variables|Default|SetIsShoot true)
  (Variables|Default|SetweaponState "VE_Shoot")
  (if (not (Variables|Default|GetwaitForEquip))
    (CallFunction|StartRaycast)
    (Components|Activation|Activate (Variables|Default|GetShaft_Laser) false)
    (bind (_outhit_location _returnvalue _outhit_traceend) (CallFunction|Raycast false))
    (if _returnvalue
      (CallFunction|SendData _outhit_location (Variables|Default|GetIsShoot))
      (else
        (CallFunction|SendData _outhit_traceend (Variables|Default|GetIsShoot))))))

(event EventTick
  (params (DeltaSeconds :type Float%20%28single-precision%29))
  (bind _shaft_laser (Variables|Default|GetShaft_Laser))
  (Variables|Default|SetDelta%20Seconds DeltaSeconds)
  (if (Variables|/Game/Game/Player/BP_Player.BP_Player_C|GetIsMine (Variables|Default|GetPlayer))
    (if (and (Variables|Default|GetIsShoot) (not (Variables|Default|GetwaitForEquip)))
      (Default|RemoveBulletfromCurrentWeapon (Variables|Default|GetPlayer) true)
      (Effects|Components|ParticleSystem|SetFloatParameter _shaft_laser "Scale" (Variables|Default|GetStartLaserScale))
      (Effects|Components|ParticleSystem|SetFloatParameter _shaft_laser "SpawnRate" 1.0)
      (bind (_outhit_location _returnvalue _outhit_traceend) (CallFunction|Raycast true))
      (if _returnvalue
        (Variables|Default|SetLastLaserPos _outhit_location)
        (Components|Activation|Activate (Variables|Default|GetHit) false)
        (else
          (Variables|Default|SetLastLaserPos _outhit_traceend)
          (Components|Activation|Deactivate (Variables|Default|GetHit))))
      (Effects|Components|ParticleSystem|SetVectorParameter (Variables|Default|GetShaft_Laser) "BeamEnd" (Variables|Default|GetLastLaserPos))
      (Effects|Components|ParticleSystem|SetVectorParameter (Variables|Default|GetHit) "HitLocation" (Variables|Default|GetLastLaserPos))
      (CallFunction|SendData (Variables|Default|GetLastLaserPos) true)
      (else
        (Effects|Components|ParticleSystem|SetFloatParameter (Variables|Default|GetShaft_Laser) "Scale" 0.0)
        (Components|Activation|Deactivate (Variables|Default|GetHit))))
    (else
      (CallFunction|UpdateLaserClient))))

(event EventOnStopShoot
  (Variables|Default|SetIsShoot false)
  (Variables|Default|SetweaponState "VE_Idle")
  (Components|Activation|Deactivate (Variables|Default|GetShaft_Laser))
  (bind (_outhit_location _returnvalue _outhit_traceend) (CallFunction|Raycast false))
  (if _returnvalue
    (CallFunction|SendData _outhit_location (Variables|Default|GetIsShoot))
    (else
      (CallFunction|SendData _outhit_traceend (Variables|Default|GetIsShoot)))))

(fn ConstructionScript)

(fn Raycast
  (params (CallDamage :type Boolean))
  (bind _player (Variables|Default|GetPlayer))
  (bind _laserdistance (Variables|Default|GetLaserDistance))
  (bind _weapondata (Variables|Default|GetWeaponData))
  (bind _player_2 (Variables|Default|GetPlayer))
  (bind _camera (Variables|/Game/Game/Player/BP_Player.BP_Player_C|GetCamera _player))
  (bind _returnvalue (Transformation|GetWorldLocation _camera))
  (bind _returnvalue_2 (Math|Vector|GetForwardVector _camera))
  (bind _returnvalue_3 (* _returnvalue_2 _laserdistance))
  (bind _returnvalue_4 (+ _returnvalue _returnvalue_3))
  (Utilities|Array|Add (LocalVariables|GetIgnored) _player_2)
  (if CallDamage
    (Default|ShootShaftDamageServer (Variables|/Game/Game/Player/BP_Player.BP_Player_C|GetBP_MultiplayerHandlerComponent _player_2) _returnvalue _returnvalue_4 (/ (Variables|/Script/ShooterRooms.WeaponDataAsset|Getdamage _weapondata) (Math|Conversions|ToFloat(Integer) (Variables|/Script/ShooterRooms.WeaponDataAsset|GettickRate _weapondata)))))
  (bind (_outhit _returnvalue_5) (Collision|LineTraceForObjects _returnvalue _returnvalue_4 (Utilities|Array|MakeArray "ObjectTypeQuery1" "ObjectTypeQuery3" "ObjectTypeQuery2") false (LocalVariables|GetIgnored) "None"))
  (return (.location _outhit) _returnvalue_5 (.traceend _outhit)))

(fn StartRaycast
  (bind (_outhit_location _returnvalue _outhit_traceend) (CallFunction|Raycast false))
  (if _returnvalue
    (Variables|Default|SetLastLaserPos _outhit_location)
    (else
      (Variables|Default|SetLastLaserPos _outhit_traceend))))

(fn SendData
  (params (Pos :type Vector) (State :type Boolean))
  (Default|ShootShaftUpdate (Variables|/Game/Game/Player/BP_Player.BP_Player_C|GetBP_MultiplayerHandlerComponent (Variables|Default|GetPlayer)) (Utilities|Struct|MakeST_ShaftStatus State Pos)))

(fn UpdateLaserClient
  (bind _shaft_laser (Variables|Default|GetShaft_Laser))
  (bind _output_get (LocalVariables|SetShaftData (Variables|/Game/Game/Player/Components/BP_MultiplayerHandlerComponent.BP_MultiplayerHandlerComponent_C|GetShaftData (Variables|/Game/Game/Player/BP_Player.BP_Player_C|GetBP_MultiplayerHandlerComponent (Variables|Default|GetPlayer)))))
  (if (!= (Variables|Default|GetIsShoot) (.isshooted _output_get))
    (Variables|Default|SetIsShoot (.isshooted _output_get))
    (if (.isshooted _output_get)
      (Components|Activation|Activate (Variables|Default|GetShaft_Laser) false)
      (else
        (Components|Activation|Deactivate (Variables|Default|GetShaft_Laser)))))
  (if (.isshooted _output_get)
    (Transformation|SetWorldLocation (Variables|Default|GetShaft_Laser) (Transformation|GetSocketLocation (Variables|/Game/Game/Player/BP_Player.BP_Player_C|GetWeapon (Variables|Default|GetPlayer)) "ClientLaserPoint") false false)
    (Effects|Components|ParticleSystem|SetFloatParameter _shaft_laser "Scale" (Variables|Default|GetStartLaserScale))
    (Effects|Components|ParticleSystem|SetFloatParameter _shaft_laser "SpawnRate" 1.0)
    (Variables|Default|SetLastLaserPos (.position (LocalVariables|GetShaftData)))
    (Components|Activation|Activate (Variables|Default|GetHit) false)
    (Effects|Components|ParticleSystem|SetVectorParameter (Variables|Default|GetShaft_Laser) "BeamEnd" (Variables|Default|GetLastLaserPos))
    (Effects|Components|ParticleSystem|SetVectorParameter (Variables|Default|GetHit) "HitLocation" (Variables|Default|GetLastLaserPos))
    (else
      (Effects|Components|ParticleSystem|SetFloatParameter (Variables|Default|GetShaft_Laser) "Scale" 1.0)
      (Components|Activation|Deactivate (Variables|Default|GetHit)))))