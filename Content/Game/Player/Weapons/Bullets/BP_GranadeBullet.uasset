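; Grenade projectile that explodes five seconds after spawn or when its sphere overlaps a player, ignoring its owner for the first 0.1 seconds.
; The authority applies weapon-data damage through BPExplosionComponent, fires a radial impulse and guards against repeat detonation with IsDead.
; ExplodeRPC activates the explosion effect, hides the grenade and disables its physics and collision.
; The light-flash timeline and its delayed DestroyActor are not connected.
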(event OnComponentBeginOverlap(Sphere_0)
  (params (OverlappedComponent :type Primitive%20Component%20Object%20Reference) (OtherActor :type Actor%20Object%20Reference) (OtherComp :type Primitive%20Component%20Object%20Reference) (OtherBodyIndex :type Integer) (bFromSweep :type Boolean) (SweepResult :type Hit%20Result%20Structure%20%28by%20ref%29))
  (bind _granade (Variables|Default|GetGranade))
  (bind _bp_explosioncomponent (Variables|Default|GetBP_ExplosionComponent))
  (Networking|SwitchHasAuthority
    (:Authority
      (if (!= (Utilities|GetClass OtherActor) "BP_GranadeBullet_C")
        (Utilities|Casting|CastToBP_Player OtherActor)
        (if (or (!= OtherActor (Components|GetOwner)) (> (Variables|Default|GetTime) 0.1))
          (if (not (Variables|Default|GetIsDead))
            (Default|SetPos _bp_explosioncomponent (Transformation|GetWorldLocation (Variables|Default|GetGranade)))
            (Default|DamagePlayer _bp_explosioncomponent (Variables|Default|GetSender))
            (Class|RadialForceComponent|FireImpulse (Variables|Default|GetRadialForce))
            (Variables|Default|SetIsDead true)
            (CallFunction|ExplodeRPC)
            (Physics|SetEnableGravity _granade false)
            (Physics|SetSimulatePhysics _granade false)
            (Collision|SetCollisionEnabled _granade "NoCollision")))))))

(event Custom|ExplodeRPC
  (bind _granade (Variables|Default|GetGranade))
  (Variables|Default|SetIsDead true)
  (Components|Activation|Activate (Variables|Default|GetExplosion) false)
  (Rendering|SetVisibility (Variables|Default|GetGranade) false false)
  (Physics|SetEnableGravity _granade false)
  (Physics|SetSimulatePhysics _granade false)
  (Collision|SetCollisionEnabled _granade "NoCollision"))

(event EventBeginPlay
  (bind _granade (Variables|Default|GetGranade))
  (bind _bp_explosioncomponent (Variables|Default|GetBP_ExplosionComponent))
  (Variables|/Game/Game/Player/Components/BP_ExplosionComponent.BP_ExplosionComponent_C|SetDamage (Variables|Default|GetBP_ExplosionComponent) (Variables|/Script/ShooterRooms.WeaponDataAsset|Getdamage (Variables|Default|GetWeaponData)))
  (Networking|SwitchHasAuthority
    (:Authority
      (Utilities|FlowControl|Delay 5.0)
      (if (not (Variables|Default|GetIsDead))
        (Default|SetPos _bp_explosioncomponent (Transformation|GetWorldLocation (Variables|Default|GetGranade)))
        (Default|DamagePlayer _bp_explosioncomponent (Variables|Default|GetSender))
        (Class|RadialForceComponent|FireImpulse (Variables|Default|GetRadialForce))
        (Variables|Default|SetIsDead true)
        (CallFunction|ExplodeRPC)
        (Physics|SetEnableGravity _granade false)
        (Physics|SetSimulatePhysics _granade false)
        (Collision|SetCollisionEnabled _granade "NoCollision")))))

(event EventTick
  (params (DeltaSeconds :type Float%20%28single-precision%29))
  (Networking|SwitchHasAuthority
    (:Authority
      (Variables|Default|SetTime (+ DeltaSeconds (Variables|Default|GetTime))))))

(fn ConstructionScript)