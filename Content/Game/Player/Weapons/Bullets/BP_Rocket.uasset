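; BP_Rocket is a rocket projectile that explodes on impact, damaging players and applying a radial impulse.
; A sphere hit, or an authority-side overlap with a non-owner, runs a one-shot sequence that stops the rocket and destroys it after a short delay.
; Damage comes from WeaponData through BPExplosionComponent, while DecalSpawn limits the decal, trail shutoff and explosion effect to the Remote branch.
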(event OnComponentHit(Sphere)
  (params (HitComponent :type Primitive%20Component%20Object%20Reference) (OtherActor :type Actor%20Object%20Reference) (OtherComp :type Primitive%20Component%20Object%20Reference) (NormalImpulse :type Vector :default "0, 0, 0") (Hit :type Hit%20Result%20Structure%20%28by%20ref%29))
  (bind _projectilemovement (Variables|Default|GetProjectileMovement))
  (Variables|Default|SetHit%20Impact%20Point (.impactpoint Hit))
  (Variables|Default|SetHit%20Impact%20Normal (.impactnormal Hit))
  (Variables|Default|SetHit%20Hit%20Component (.hitcomponent Hit))
  (if (not (Variables|Default|GetIsDead))
    (Variables|Default|SetIsDead true)
    (Variables|/Script/Engine.ProjectileMovementComponent|SetMaxSpeed _projectilemovement 0.0)
    (Variables|/Script/Engine.MovementComponent|SetVelocity _projectilemovement "0, 0, 0")
    (CallFunction|DecalSpawn)
    (Components|DestroyComponent (Variables|Default|GetProjectileMovement))
    (Components|DestroyComponent (Variables|Default|GetRocket))
    (Class|RadialForceComponent|FireImpulse (Variables|Default|GetRadialForce))
    (Default|DamagePlayer (Variables|Default|GetBP_ExplosionComponent) (Variables|Default|GetSender))
    (Utilities|FlowControl|Delay 2.0)
    (Actor|DestroyActor)))

(event OnComponentBeginOverlap(Sphere)
  (params (OverlappedComponent :type Primitive%20Component%20Object%20Reference) (OtherActor :type Actor%20Object%20Reference) (OtherComp :type Primitive%20Component%20Object%20Reference) (OtherBodyIndex :type Integer) (bFromSweep :type Boolean) (SweepResult :type Hit%20Result%20Structure%20%28by%20ref%29))
  (bind _projectilemovement (Variables|Default|GetProjectileMovement))
  (Networking|SwitchHasAuthority
    (:Authority
      (if (!= OtherActor (Components|GetOwner))
        (Variables|Default|SetHit%20Impact%20Point (.impactpoint SweepResult))
        (Variables|Default|SetHit%20Impact%20Normal (.normal SweepResult))
        (Variables|Default|SetHit%20Hit%20Component OtherComp)
        (if (not (Variables|Default|GetIsDead))
          (Variables|Default|SetIsDead true)
          (Variables|/Script/Engine.ProjectileMovementComponent|SetMaxSpeed _projectilemovement 0.0)
          (Variables|/Script/Engine.MovementComponent|SetVelocity _projectilemovement "0, 0, 0")
          (CallFunction|DecalSpawn)
          (Components|DestroyComponent (Variables|Default|GetProjectileMovement))
          (Components|DestroyComponent (Variables|Default|GetRocket))
          (Class|RadialForceComponent|FireImpulse (Variables|Default|GetRadialForce))
          (Default|DamagePlayer (Variables|Default|GetBP_ExplosionComponent) (Variables|Default|GetSender))
          (Utilities|FlowControl|Delay 2.0)
          (Actor|DestroyActor))))))

(event Custom|DecalSpawn
  (Networking|SwitchHasAuthority
    (:Remote
      (CallFunction|SpawnDecal (Variables|Default|GetHit%20Hit%20Component) (Variables|Default|GetHit%20Impact%20Point) (Math|Conversions|RotationFromXVector (Variables|Default|GetHit%20Impact%20Normal)) (Math|Random|RandomFloatinRange 2e+01 3e+01) "/Game/Game/Player/Data/Decals/DA_ExplodeDecal.DA_ExplodeDecal")
      (Effects|Components|ParticleSystem|SetFloatParameter (Variables|Default|GetNiagara) "SpawnRateValue" 0.0)
      (Components|Activation|Activate (Variables|Default|GetExplode) true))))

(event EventBeginPlay
  (Variables|/Game/Game/Player/Components/BP_ExplosionComponent.BP_ExplosionComponent_C|SetDamage (Variables|Default|GetBP_ExplosionComponent) (Variables|/Script/ShooterRooms.WeaponDataAsset|Getdamage (Variables|Default|GetWeaponData))))

(fn ConstructionScript)