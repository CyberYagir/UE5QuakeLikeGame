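; Weapon projectile that damages players and leaves a hole decal on impact.
; Overlapping a player other than its owner applies the weapon data's damage through their stats component, then joins the shared impact path used by blocking hits.
; Impact runs once, halting movement, animating actor scale on a timeline and destroying the actor.
; Only non-authority instances spawn the decal and zero the Niagara spawn rate.
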(event OnComponentBeginOverlap(Sphere)
  (params (OverlappedComponent :type Primitive%20Component%20Object%20Reference) (OtherActor :type Actor%20Object%20Reference) (OtherComp :type Primitive%20Component%20Object%20Reference) (OtherBodyIndex :type Integer) (bFromSweep :type Boolean) (SweepResult :type Hit%20Result%20Structure%20%28by%20ref%29))
  (bind _projectilemovement (Variables|Default|GetProjectileMovement))
  (if (!= OtherActor (Components|GetOwner))
    (bind _asbp_player (Utilities|Casting|CastToBP_Player OtherActor))
    (Default|TakeDamage (Variables|/Game/Game/Player/BP_Player.BP_Player_C|GetBP_StatsComponent _asbp_player) (Variables|/Script/ShooterRooms.WeaponDataAsset|Getdamage (Variables|Default|GetWeaponData)) "NewEnumerator3" (Variables|Default|GetSender))
    (Variables|Default|SetHit%20Impact%20Point (.impactpoint SweepResult))
    (Variables|Default|SetHit%20Impact%20Normal (.normal SweepResult))
    (Variables|Default|SetHit%20Hit%20Component OtherComp)
    (if (not (Variables|Default|GetIsDead))
      (Variables|Default|SetIsDead true)
      (Variables|/Script/Engine.ProjectileMovementComponent|SetMaxSpeed _projectilemovement 0.0)
      (Variables|/Script/Engine.MovementComponent|SetVelocity _projectilemovement "0, 0, 0")
      (CallFunction|DecalSpawn)
      (bind _scale (Timeline|Timeline Play)
        (:Update
          (Transformation|SetActorScale3D (* (Math|Vector|MakeVector 1.0 1.0 1.0) _scale)))
        (:Finished
          (Actor|DestroyActor))))))

(event OnComponentHit(Sphere)
  (params (HitComponent :type Primitive%20Component%20Object%20Reference) (OtherActor :type Actor%20Object%20Reference) (OtherComp :type Primitive%20Component%20Object%20Reference) (NormalImpulse :type Vector :default "0, 0, 0") (Hit :type Hit%20Result%20Structure%20%28by%20ref%29))
  (bind _projectilemovement (Variables|Default|GetProjectileMovement))
  (Variables|Default|SetHit%20Impact%20Point (.impactpoint Hit))
  (Variables|Default|SetHit%20Impact%20Normal (.impactnormal Hit))
  (Variables|Default|SetHit%20Hit%20Component (.hitcomponent Hit))
  (if (not (Variables|Default|GetIsDead))
    (Variables|Default|SetIsDead true)
    (Variables|/Script/Engine.ProjectileMovementComponent|SetMaxSpeed _projectilemovement 0.0)
    (Variables|/Script/Engine.MovementComponent|SetVelocity _projectilemovement "0, 0, 0")
    (CallFunction|DecalSpawn)
    (bind _scale (Timeline|Timeline Play)
      (:Update
        (Transformation|SetActorScale3D (* (Math|Vector|MakeVector 1.0 1.0 1.0) _scale)))
      (:Finished
        (Actor|DestroyActor)))))

(event Custom|DecalSpawn
  (Networking|SwitchHasAuthority
    (:Remote
      (CallFunction|SpawnDecal (Variables|Default|GetHit%20Hit%20Component) (Variables|Default|GetHit%20Impact%20Point) (Math|Conversions|RotationFromXVector (Variables|Default|GetHit%20Impact%20Normal)) 3.0 "/Game/Game/Player/Data/Decals/DA_HoleDecal.DA_HoleDecal")
      (Effects|Components|ParticleSystem|SetFloatParameter (Variables|Default|GetNiagara) "SpawnRateValue" 0.0))))

(fn ConstructionScript)