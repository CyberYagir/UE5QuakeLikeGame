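; BP_GanadeLuncher is a player weapon Blueprint for a grenade launcher.
; On shoot, it removes a bullet from the player's current weapon and activates its Niagara effect.
; It then asks the player's multiplayer handler component to spawn the shot through ShootGranadeServer, passing the Point component's transform, forward vector and a Force value.
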(event EventOnShootBullets
  (bind _point (Variables|Default|GetPoint))
  (Default|RemoveBulletfromCurrentWeapon (Variables|Default|GetPlayer) false)
  (Components|Activation|Activate (Variables|Default|GetNiagara) true)
  (Default|ShootGranadeServer (Variables|/Game/Game/Player/BP_Player.BP_Player_C|GetBP_MultiplayerHandlerComponent (Variables|Default|GetPlayer)) (Transformation|GetWorldTransform _point) (Math|Vector|GetForwardVector _point) (Variables|Default|GetForce)))

(fn ConstructionScript)