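; Rocket launcher weapon Blueprint that handles firing a rocket for the player.
; On each shot it removes a round from the current weapon, launches the projectile and activates the muzzle effect.
; Aim comes from a camera trace with random spread, ignoring the owner and player.
; The muzzle point transform, rotated toward the hit or trace end, goes to the player's multiplayer handler to request the rocket through ShootRocketServer.
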(event EventOnShootBullets
  (Default|RemoveBulletfromCurrentWeapon (Variables|Default|GetPlayer) false)
  (CallFunction|ShootProjectile)
  (Components|Activation|Activate (Variables|Default|GetShotgun_Muzzle) true))

(fn ConstructionScript)

(fn ShootProjectile
  (bind _point (Variables|Default|GetPoint))
  (bind _returnvalue (Transformation|GetWorldTransform _point))
  (bind (_location _rotation _scale) (Math|Transform|BreakTransform _returnvalue))
  (bind _asbp_player (Utilities|Casting|CastToBP_Player (Game|GetPlayerCharacter 0)))
  (LocalVariables|SetIgnored (Utilities|Array|MakeArray (Components|GetOwner) _asbp_player))
  (LocalVariables|SetCamera (Variables|/Game/Game/Player/BP_Player.BP_Player_C|GetCamera _asbp_player))
  (bind _returnvalue_2 (CallFunction|CreateRandomRotator))
  (bind _output_get (LocalVariables|SetEndPos (+ (Transformation|GetWorldLocation (LocalVariables|GetCamera)) (* (Math|Vector|GetForwardVector (Math|Rotator|CombineRotators (Transformation|GetWorldRotation (LocalVariables|GetCamera)) _returnvalue_2)) 10000))))
  (bind (_outhit _returnvalue_3) (Collision|LineTraceByChannel (Transformation|GetWorldLocation (LocalVariables|GetCamera)) _output_get "TraceTypeQuery1" false (LocalVariables|GetIgnored) "None"))
  (if _returnvalue_3
    (LocalVariables|SetEndPos (.Location (Collision|BreakHitResult _outhit))))
  (Default|ShootRocketServer (Variables|/Game/Game/Player/BP_Player.BP_Player_C|GetBP_MultiplayerHandlerComponent (Variables|Default|GetPlayer)) (Math|Transform|MakeTransform _location (Math|Rotator|FindLookatRotation _location (LocalVariables|GetEndPos)) _scale)))