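; Base weapon Blueprint for the player, driving equip, idle, shoot and de-equip through montages and a weapon state.
; It finds BP_Player through its parent component's owner and blocks shooting until equipping completes.
; Shooting calls an empty OnShootBullets hook and returns to a repeating idle when the montage completes; de-equipping ends in OnDequipEnd.
; Helpers provide random spread rotations, randomly rolled impact decals and mesh hiding.
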(event Custom|OnShootBullets)

(event Custom|OnDequipEnd)

(event EventBeginPlay
  (CallFunction|GetPlayer)
  (Variables|Default|SetweaponState "VE_Idle")
  (Variables|Default|SetwaitForEquip true)
  (Animation|Montage|PlayMontage (Variables|Default|GetSkeletalMesh) (Variables|Default|GetEquip_Montage)
    (:OnCompleted
      (Variables|Default|SetwaitForEquip false)
      (Animation|Montage|PlayMontage (Variables|Default|GetSkeletalMesh) (Variables|Default|GetIdle_Montage)))))

(event EventDeEquip
  (Variables|Default|SetweaponState "VE_Dequip")
  (Animation|Montage|PlayMontage (Variables|Default|GetSkeletalMesh) (Variables|Default|GetDeEquip_Montage)
    (:OnCompleted
      (CallFunction|OnDequipEnd))))

(event EventOnStopShoot)

(event EventOnShoot
  (if (and (Utilities|Enum|Equal(Enum) (Variables|Default|GetweaponState) "VE_Idle") (not (Variables|Default|GetwaitForEquip)))
    (Variables|Default|SetweaponState "VE_Shoot")
    (CallFunction|OnShootBullets)
    (Animation|Montage|PlayMontage (Variables|Default|GetSkeletalMesh) (Variables|Default|GetShoot_Montage)
      (:OnCompleted
        (Variables|Default|SetweaponState "VE_Idle" :!label _label)
        (Animation|Montage|PlayMontage (Variables|Default|GetSkeletalMesh) (Variables|Default|GetIdle_Montage)
          (:OnCompleted
            (goto _label)))))))

(fn ConstructionScript)

(fn SetupWeapon
  (params (EquipMontage :type Anim%20Montage%20Object%20Reference) (IdleMontage :type Anim%20Montage%20Object%20Reference)))

(fn SpawnDecal
  (params (AttachToComponent :type Scene%20Component%20Object%20Reference) (Location :type Vector) (Rotation :type Rotator) (Scale :type Float%20%28double-precision%29))
  (bind _returnvalue (Class|GameplayStatics|SpawnDecalAttached (.OutItem (Utilities|Array|Random (Variables|Default|GetDecalsArray))) (* Scale (Math|Vector|MakeVector 2.0 4.0 4.0)) AttachToComponent "None" Location Rotation "KeepWorldPosition" 1e+01))
  (Rendering|Components|Decal|SetFadeScreenSize _returnvalue 0.001)
  (Transformation|AddRelativeRotation _returnvalue (Math|Rotator|MakeRotator (Math|Random|RandomFloatinRange 0.0 3.6e+02) 0.0 0.0) false false))

(fn CreateRandomRotator
  (bind _spreadangle (Variables|Default|GetSpreadAngle))
  (bind _spreadangle_2 (Variables|Default|GetSpreadAngle))
  (bind _returnvalue (* _spreadangle_2 -1.0))
  (return (Math|Rotator|MakeRotator (Math|Random|RandomFloatinRange _returnvalue _spreadangle) (Math|Random|RandomFloatinRange _returnvalue _spreadangle) (Math|Random|RandomFloatinRange _returnvalue _spreadangle))))

(fn GetPlayer
  (bind _asbp_player (Utilities|Casting|CastToBP_Player (Components|GetOwner (Class|Actor|GetParentComponent))))
  (Variables|Default|SetPlayer _asbp_player))

(fn DisableMesh
  (Rendering|SetVisibility (Variables|Default|GetSkeletalMesh) false false))