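; Free-fly spectator pawn that lets a player roam until the respawn timer expires, then respawn with Space.
; Floating movement supports vertical flight and a speed boost that widens camera FOV.
; The controlling client relays position changes through LerpRPC, and other clients interpolate toward them.
; Init builds timer, respawn and score UI, while a locally controlled authority instead gets host text, disabled rendering and 800x600 resolution.
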(event Custom|LerpRPC
  (params (NewPos :type Vector))
  (if (not (Pawn|IsLocallyControlled))
    (Variables|Default|SetLerpLocaiton NewPos)))

(event Custom|Init
  (params (Player :type BP%20Player%20State%20Object%20Reference) (Transform :type Transform))
  (Variables|Default|SetPlayer Player)
  (bind _asbp_player_controller (Utilities|Casting|CastToBP_PlayerController (Pawn|GetController)))
  (bind _output_get (Variables|Default|SetAs%20BP%20Player%20Controller _asbp_player_controller))
  (if (Pawn|IsLocallyControlled)
    (Pawn|SetControlRotation _output_get (.rotation Transform))
    (CallFunction|UIConstruct)))

(event Custom|ChangePositionCommand
  (params (NewPos :type Vector))
  (CallFunction|LerpRPC NewPos))

(event EventTick
  (params (DeltaSeconds :type Float%20%28single-precision%29))
  (bind _returnvalue (Transformation|GetActorLocation))
  (Networking|SwitchHasAuthority
    (:Remote
      (if (Pawn|IsLocallyControlled)
        (CallFunction|FovAnimation)
        (if (Utilities|Operators|NotEqual(!=) _returnvalue (Variables|Default|GetOldPos) 0.1)
          (CallFunction|ChangePositionCommand _returnvalue))
        (else
          (Transformation|SetActorLocation (Math|Vector|Lerp(Vector) (Transformation|GetActorLocation) (Variables|Default|GetLerpLocaiton) (* DeltaSeconds 1e+01)) false false))))))

(event Input|KeyboardEvents|SpaceBar
  (params (Key :type Key%20Structure :default "None"))
  (bind _as_bp_player_controller (Variables|Default|GetAs%20BP%20Player%20Controller))
  (:Pressed
    (bind _returnvalue (Default|GetTime (Variables|Default|GetPlayer)))
    (if (<= _returnvalue 0)
      (Default|SetActive (Variables|/Game/Game/Player/BP_PlayerController.BP_PlayerController_C|GetUI_Respawn _as_bp_player_controller) false)
      (Default|SpawnPlayer _as_bp_player_controller))))

(event Input|AxisEvents|InputAxisBoost
  (params (AxisValue :type Float%20%28single-precision%29))
  (bind _movement (Variables|Default|GetMovement))
  (if (> AxisValue 0.0)
    (Variables|/Script/Engine.FloatingPawnMovement|SetMaxSpeed _movement (* (Variables|Default|GetSpeed) 1.5))
    (else
      (Variables|/Script/Engine.FloatingPawnMovement|SetMaxSpeed _movement (Variables|Default|GetSpeed)))))

(event Input|AxisEvents|InputAxisHorizontal
  (params (AxisValue :type Float%20%28single-precision%29))
  ;[1 0 0.3281] Move
  (Pawn|Input|AddMovementInput (Transformation|GetActorRightVector) AxisValue false))

(event Input|AxisEvents|InputAxisJump
  (params (AxisValue :type Float%20%28single-precision%29))
  (Pawn|Input|AddMovementInput (Transformation|GetActorUpVector) AxisValue false))

(event Input|AxisEvents|InputAxisMoveDown
  (params (AxisValue :type Float%20%28single-precision%29))
  (Pawn|Input|AddMovementInput (Transformation|GetActorUpVector) (* AxisValue -1.0) false))

(event Input|AxisEvents|InputAxisMouse_Y
  (params (AxisValue :type Float%20%28single-precision%29))
  ;[0 0.9062 1] Look
  (Pawn|Input|AddControllerPitchInput (* AxisValue -1.0)))

(event Input|AxisEvents|InputAxisMouse_X
  (params (AxisValue :type Float%20%28single-precision%29))
  ;[0 0.9062 1] Look
  (Pawn|Input|AddControllerYawInput AxisValue))

(event Input|AxisEvents|InputAxisForward
  (params (AxisValue :type Float%20%28single-precision%29))
  ;[1 0 0.3281] Move
  (Pawn|Input|AddMovementInput (Transformation|GetActorForwardVector) AxisValue false))

(fn ConstructionScript
  (bind _output_get (Variables|Default|SetMovement (Variables|Default|GetFloatingPawnMovement)))
  (Variables|/Script/Engine.FloatingPawnMovement|SetMaxSpeed _output_get (Variables|Default|GetSpeed)))

(fn DestroyMovement
  (Components|DestroyComponent (Variables|Default|GetMovement)))

(fn AddMovement
  (bind _returnvalue (AddComponent|AddFloatingPawnMovement))
  (Variables|Default|SetMovement _returnvalue))

(fn FovAnimation
  (Camera|SetFieldOfView (Variables|Default|GetCamera) (Math|Float|Lerp 9e+01 1e+02 (/ (Math|Float|Clamp(Float) (- (Math|Vector|VectorLength (Variables|/Script/Engine.MovementComponent|GetVelocity (Variables|Default|GetMovement))) (Variables|Default|GetSpeed)) 0.0 9999.0) (- (* (Variables|Default|GetSpeed) 1.5) (Variables|Default|GetSpeed))))))

(fn UIConstruct
  (Utilities|FlowControl|Sequence
    (:then_0
      (Utilities|IsValid (Variables|/Game/Game/Player/BP_PlayerController.BP_PlayerController_C|GetUI_Timer (Variables|Default|GetAs%20BP%20Player%20Controller))
        (:Is%20Valid
          (Variables|/Script/UMG.Widget|SetVisibility (Variables|/Game/Game/Player/BP_PlayerController.BP_PlayerController_C|GetUI_Timer (Variables|Default|GetAs%20BP%20Player%20Controller)) "Visible"))
        (:Is%20Not%20Valid
          (bind _returnvalue (Game|ConstructObjectfromClass "/Game/Game/Player/UI/BP_Timer.BP_Timer_C"))
          (UserInterface|Viewport|AddtoViewport _returnvalue 0)
          (Variables|/Game/Game/Player/BP_PlayerController.BP_PlayerController_C|SetUI_Timer (Variables|Default|GetAs%20BP%20Player%20Controller) _returnvalue))))
    (:then_1
      (Utilities|IsValid (Variables|/Game/Game/Player/BP_PlayerController.BP_PlayerController_C|GetUI_Respawn (Variables|Default|GetAs%20BP%20Player%20Controller))
        (:Is%20Valid
          (Default|SetActive (Variables|/Game/Game/Player/BP_PlayerController.BP_PlayerController_C|GetUI_Respawn (Variables|Default|GetAs%20BP%20Player%20Controller)) true))
        (:Is%20Not%20Valid
          (Networking|SwitchHasAuthority
            (:Authority
              (bind _returnvalue_2 (Game|ConstructObjectfromClass "/Game/Game/Player/UI/BP_HostText.BP_HostText_C"))
              (UserInterface|Viewport|AddtoViewport _returnvalue_2 0)
              (Class|MyBlueprintFunctionLibrary|DisableRendering self)
              (bind _returnvalue_3 (Settings|GetGameUserSettings))
              (Class|GameUserSettings|SetScreenResolution _returnvalue_3 (Utilities|Struct|MakeIntPoint 800 600))
              (Class|GameUserSettings|ApplyResolutionSettings _returnvalue_3 false))
            (:Remote
              (bind _returnvalue_4 (Game|ConstructObjectfromClass "/Game/Game/Player/UI/BP_RespawnTimer.BP_RespawnTimer_C"))
              (bind _output_get (Variables|Default|SetRespawnUI _returnvalue_4))
              (Default|Init _output_get (Variables|Default|GetPlayer))
              (UserInterface|Viewport|AddtoViewport _output_get 0)
              (Variables|/Game/Game/Player/BP_PlayerController.BP_PlayerController_C|SetUI_Respawn (Variables|Default|GetAs%20BP%20Player%20Controller) _output_get))))))
    (:then_2
      (Utilities|IsValid (Variables|/Game/Game/Player/BP_PlayerController.BP_PlayerController_C|GetUI_Scores (Variables|Default|GetAs%20BP%20Player%20Controller))
        (:Is%20Not%20Valid
          (bind _returnvalue_5 (Game|ConstructObjectfromClass "/Game/Game/Player/UI/BP_Scorelist_UI.BP_Scorelist_UI_C"))
          (UserInterface|Viewport|AddtoViewport _returnvalue_5 0)
          (bind _output_get_2 (Variables|/Game/Game/Player/BP_PlayerController.BP_PlayerController_C|SetUI_Scores (Variables|Default|GetAs%20BP%20Player%20Controller) _returnvalue_5))
          (Variables|/Script/UMG.Widget|SetVisibility _output_get_2 "Hidden"))))))