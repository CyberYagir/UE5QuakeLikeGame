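; Multiplayer game mode that runs timed rounds, tracks connected players and spawns their player, spectator and end-game pawns.
; A self-rearming one-second timer updates the game state clock and advances each player's respawn timer.
; At time-up it removes pawns, shows the end-game preview, then after a delay resets scores and restarts.
; Kill, death and score stats for non-local controllers live in a struct array copied to BP_GameStateBase.
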(event Custom|StartTimer
  ;[1 0 0.5156] Timer
  (Server|ResetServer)
  (Scores|ResetSpawnTimers)
  (Utilities|Time|SetTimerbyEvent (delegate Custom|MatchTimerFuction) 1.0)
  (Variables|Default|SetMatchTimerHandle "")
  (Math|Integer|IncrementInt (Variables|Default|GetTimerSeconds)))

(event Custom|MatchTimerFuction
  ;[1 0 0.5156] Timer
  ;;[0.1719 1 0] Check Timer Is End
  (Default|UpdateMatchTimer (Variables|Default|GetAs%20BP%20Game%20State%20Base) (Variables|Default|GetTimerSeconds))
  (if (>= (Variables|Default|GetTimerSeconds) (Variables|Default|GetMaxMatchTime))
    ;[0.007812 0 1] End Game
    (Utilities|Time|ClearandInvalidateTimerbyHandle (Variables|Default|GetMatchTimerHandle))
    (CallFunction|ChangeRoundState "NewEnumerator1")
    (Spawn|RemoveAllControllers)
    (CallFunction|SeeEndGamePreview true)
    (Utilities|FlowControl|Delay 1e+01)
    (Scores|ResetScores)
    (CallFunction|ChangeRoundState "NewEnumerator1")
    (CallFunction|SeeEndGamePreview false)
    (Spawn|SpawnAllSpectrators)
    (CallFunction|StartTimer)
    (else
      ;[1 0 0.6797] Every Second Tick
      (for _array_element (Variables|Default|GetPlayersList)
        (bind _asbp_player_state (Utilities|Casting|CastToBP_PlayerState (Variables|/Script/Engine.Controller|GetPlayerState _array_element)))
        (Math|Integer|IncrementInt (Variables|/Game/Game/Player/BP_PlayerState.BP_PlayerState_C|GetRespawnTimer _asbp_player_state)))
      (Utilities|Time|SetTimerbyEvent (delegate Custom|MatchTimerFuction) 1.0)
      (Variables|Default|SetMatchTimerHandle "")
      (Math|Integer|IncrementInt (Variables|Default|GetTimerSeconds)))))

(event EventOnLogout
  (params (ExitingController :type Controller%20Object%20Reference))
  ;[0 0.3203 1] Logout
  (bind _asplayer_controller (Utilities|Casting|CastToPlayerController ExitingController))
  (if (Utilities|Enum|Equal(Enum) (Variables|Default|GetRoundState) "NewEnumerator0")
    (Utilities|Array|RemoveItem (Variables|Default|GetPlayersList) _asplayer_controller)
    (bind (_array_element _array_index) (Utilities|Array|ForEachLoopwithBreak (Variables|Default|GetPlayersStats) :!label _label)
      (:LoopBody
        (if (== (.controller _array_element) _asplayer_controller)
          (Utilities|Array|RemoveIndex (Variables|Default|GetPlayersStats) _array_index)
          (goto _label Break)))
      (:Completed
        (Scores|ApplyScores)))))

(event EventPostLogin
  (params (NewPlayer :type Player%20Controller%20Object%20Reference))
  ;[1 0.75 0] Log In
  (Utilities|Array|Add (Variables|Default|GetPlayersList) NewPlayer)
  (bind _asbp_player_controller (Utilities|Casting|CastToBP_PlayerController NewPlayer))
  (if (Utilities|Enum|Equal(Enum) (Variables|Default|GetRoundState) "NewEnumerator0")
    (if (Pawn|IsLocalController _asbp_player_controller)
      _
      (else
        (Utilities|Array|Add (Variables|Default|GetPlayersStats) (Utilities|Struct|MakeST_PlayerStas _asbp_player_controller "None"))))
    (bind _asbp_game_state_base (Utilities|Casting|CastToBP_GameStateBase (Game|GetGameState)))
    (Variables|Default|SetAs%20BP%20Game%20State%20Base _asbp_game_state_base)
    (Scores|ApplyScores)
    (else
      (Default|SetEndPreview _asbp_player_controller))))

(event EventBeginPlay
  (CallFunction|StartTimer))

(fn ConstructionScript)

(fn FindSpawn
  (bind _outactors (Actor|GetAllActorsOfClass "/Script/Engine.PlayerStart"))
  (return (Transformation|GetActorTransform (.OutItem (Utilities|Array|Random _outactors)))))

(fn SpawnSpectrator
  (params (PlayerController :type Player%20Controller%20Object%20Reference))
  (bind _returnvalue (Pawn|GetControlledPawn PlayerController))
  (LocalVariables|SetPlayer PlayerController)
  (Utilities|IsValid _returnvalue
    (:Is%20Valid
      (Actor|DestroyActor _returnvalue))
    (:Is%20Not%20Valid
      _))
  (Spawn|SpawnSpetratoronPose (LocalVariables|GetPlayer) (Spawn|FindSpawn)))

(fn SpawnPlayer
  (params (PlayerController :type Player%20Controller%20Object%20Reference))
  (bind _returnvalue (Pawn|GetControlledPawn PlayerController))
  (LocalVariables|SetPlayer PlayerController)
  (Utilities|IsValid _returnvalue
    (:Is%20Valid
      (Actor|DestroyActor _returnvalue)
      (bind _output_get (LocalVariables|SetSpawnPoint (Spawn|FindSpawn))))
    (:Is%20Not%20Valid
      _))
  (bind _returnvalue_2 (Game|SpawnActorfromClass "/Game/Game/Player/BP_Player.BP_Player_C" _output_get "AlwaysSpawn" "MultiplyWithRoot" 0 0))
  (Pawn|Possess (LocalVariables|GetPlayer) _returnvalue_2)
  (Default|RotateRPCStart _returnvalue_2 (LocalVariables|GetSpawnPoint)))

(fn SpawnSpetratoronPose
  (params (PlayerController :type Player%20Controller%20Object%20Reference) (SpawnTransform :type Transform))
  (bind _output_get (LocalVariables|SetPlayer PlayerController))
  (bind _returnvalue (Game|SpawnActorfromClass "/Game/Game/Player/BP_Spectrator.BP_Spectrator_C" SpawnTransform "AlwaysSpawn" "MultiplyWithRoot" _output_get 0))
  (Pawn|Possess (LocalVariables|GetPlayer) _returnvalue)
  (bind _asbp_player_state (Utilities|Casting|CastToBP_PlayerState (Variables|/Script/Engine.Controller|GetPlayerState (LocalVariables|GetPlayer))))
  (Default|Init _returnvalue _asbp_player_state SpawnTransform)
  (Development|PrintString "Hello"))

(fn SetPlayerName
  (params (Player :type Player%20Controller%20Object%20Reference) (Name :type Name))
  (bind (_array_element _array_index) (Utilities|Array|ForEachLoopwithBreak (Variables|Default|GetPlayersStats) :!label _label)
    (:LoopBody
      (if (== (.Controller (Utilities|Struct|BreakST_PlayerStas _array_element)) Player)
        (Utilities|Array|SetArrayElem (Variables|Default|GetPlayersStats) _array_index (Utilities|Struct|MakeST_PlayerStas (.Controller (Utilities|Struct|BreakST_PlayerStas _array_element)) Name))
        (goto _label Break)))
    (:Completed
      (Variables|/Game/Game/Player/BP_GameStateBase.BP_GameStateBase_C|SetPlayersStats (Variables|Default|GetAs%20BP%20Game%20State%20Base) (Variables|Default|GetPlayersStats)))))

(fn AddKill
  (params (PlayerContr :type BP%20Player%20Controller%20Object%20Reference))
  (bind (_array_index _array_element) (CallFunction|FindPlayer PlayerContr))
  (if (!= _array_index -1)
    (Utilities|Array|SetArrayElem (Variables|Default|GetPlayersStats) _array_index (Utilities|Struct|MakeST_PlayerStas (.Controller (Utilities|Struct|BreakST_PlayerStas _array_element)) (.Name (Utilities|Struct|BreakST_PlayerStas _array_element)) (+ (.Kills (Utilities|Struct|BreakST_PlayerStas _array_element)) 1) (.Deaths (Utilities|Struct|BreakST_PlayerStas _array_element)) (.Scores (Utilities|Struct|BreakST_PlayerStas _array_element)) (.Team (Utilities|Struct|BreakST_PlayerStas _array_element))))))

(fn FindPlayer
  (params (Controller :type BP%20Player%20Controller%20Object%20Reference))
  (bind (_array_element _array_index) (Utilities|Array|ForEachLoopwithBreak (Variables|Default|GetPlayersStats))
    (:LoopBody
      (if (== (.Controller (Utilities|Struct|BreakST_PlayerStas _array_element)) Controller)
        (return _array_index _array_element)))
    (:Completed
      (return -1 ""))))

(fn AddDeath
  (params (PlayerContr :type BP%20Player%20Controller%20Object%20Reference))
  (bind (_array_index _array_element) (CallFunction|FindPlayer PlayerContr))
  (if (!= _array_index -1)
    (bind _structout (Utilities|Struct|SetmembersinST_PlayerStas _array_element (+ (.Deaths (Utilities|Struct|BreakST_PlayerStas _array_element)) 1)))
    (Utilities|Array|SetArrayElem (Variables|Default|GetPlayersStats) _array_index _structout)))

(fn AddScore
  (params (PlayerContr :type BP%20Player%20Controller%20Object%20Reference) (Val :type Integer))
  (bind (_array_index _array_element) (CallFunction|FindPlayer PlayerContr))
  (if (!= _array_index -1)
    (bind _structout (Utilities|Struct|SetmembersinST_PlayerStas _array_element (+ (.Scores (Utilities|Struct|BreakST_PlayerStas _array_element)) Val)))
    (Utilities|Array|SetArrayElem (Variables|Default|GetPlayersStats) _array_index _structout)))

(fn ApplyScores
  (Variables|/Game/Game/Player/BP_GameStateBase.BP_GameStateBase_C|SetPlayersStats (Variables|Default|GetAs%20BP%20Game%20State%20Base) (Variables|Default|GetPlayersStats)))

(fn RemoveAllControllers
  (for _array_element (Variables|Default|GetPlayersList)
    (Utilities|IsValid (Pawn|GetControlledPawn _array_element)
      (:Is%20Valid
        (Actor|DestroyActor (Pawn|GetControlledPawn _array_element))
        (bind _asbp_player_controller (Utilities|Casting|CastToBP_PlayerController _array_element))
        (Default|DisableUI _asbp_player_controller)))))

(fn ChangeRoundState
  (params (State :type E_RoundState%20Enum :default "NewEnumerator0"))
  (bind _output_get (Variables|Default|SetRoundState State))
  (Variables|/Game/Game/Player/BP_GameStateBase.BP_GameStateBase_C|SetGameState (Variables|Default|GetAs%20BP%20Game%20State%20Base) _output_get))

(fn SeeEndGamePreview
  (params (State :type Boolean))
  (bind _outactors (Actor|GetAllActorsOfClass "/Game/Game/Level/BP_EndGameSpawn.BP_EndGameSpawn_C"))
  (Default|SetPreview (Utilities|Array|Get(acopy) _outactors) State)
  (if State
    (for _array_element (Variables|Default|GetPlayersList)
      (bind _asbp_player_controller (Utilities|Casting|CastToBP_PlayerController _array_element))
      (Default|SetEndPreview _asbp_player_controller))))

(fn SpawnEndGameController
  (params (PlayerController :type Player%20Controller%20Object%20Reference) (Transform :type Transform))
  (bind _returnvalue (Pawn|GetControlledPawn PlayerController))
  (LocalVariables|SetPlayer PlayerController)
  (Utilities|IsValid _returnvalue
    (:Is%20Valid
      (Actor|DestroyActor _returnvalue))
    (:Is%20Not%20Valid
      _))
  (bind _returnvalue_2 (Game|SpawnActorfromClass "/Game/Game/Player/BP_EndGameController.BP_EndGameController_C" Transform "AlwaysSpawn" "MultiplyWithRoot" 0 0))
  (Pawn|Possess (LocalVariables|GetPlayer) _returnvalue_2))

(fn ResetScores
  (Utilities|Array|Clear (Variables|Default|GetPlayersStats))
  (for _array_element (Variables|Default|GetPlayersList)
    (bind _asbp_player_controller (Utilities|Casting|CastToBP_PlayerController _array_element))
    (if (not (Pawn|IsLocalController _asbp_player_controller))
      (Utilities|Array|Add (Variables|Default|GetPlayersStats) (Utilities|Struct|MakeST_PlayerStas _asbp_player_controller (Variables|/Game/Game/Player/BP_PlayerController.BP_PlayerController_C|GetPlayerName _asbp_player_controller)))))
  (Scores|ApplyScores))

(fn SpawnAllSpectrators
  (for _array_element (Variables|Default|GetPlayersList)
    (Utilities|IsValid (Pawn|GetControlledPawn _array_element)
      (:Is%20Valid
        (Spawn|SpawnSpectrator _array_element)))))

(fn ResetSpawnTimers
  (for _array_element (Variables|Default|GetPlayersList)
    (Utilities|IsValid _array_element
      (:Is%20Valid
        (bind _asbp_player_state (Utilities|Casting|CastToBP_PlayerState (Variables|/Script/Engine.Controller|GetPlayerState _array_element)))
        (Variables|/Game/Game/Player/BP_PlayerState.BP_PlayerState_C|SetRespawnTimer _asbp_player_state (Variables|/Game/Game/Player/BP_PlayerState.BP_PlayerState_C|GetMaxRespawnTime _asbp_player_state))))))

(fn ResetServer
  (bind _returnvalue (CallFunction|GetServerOptions))
  (bind (_servername _roundtime _maxplayers _mapname _gametype) (Utilities|Struct|BreakServerOptions _returnvalue))
  (Variables|Default|SetMaxMatchTime _roundtime)
  (Variables|Default|SetTimerSeconds 0)
  (Variables|Default|SetRoundState "NewEnumerator0")
  (Variables|Default|SetGameType _gametype)
  (bind _outactors (Actor|GetAllActorsOfClass "/Game/Game/Level/BP_PickUp.BP_PickUp_C"))
  (for _array_element _outactors
    (Default|Reset _array_element)))