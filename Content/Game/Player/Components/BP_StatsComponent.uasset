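; Player stats component that manages health and armor, pickup-style point gains, damage and death scoring in what appears to be a networked shooter.
; AddPoints clamps to normal or buffed caps; the owning player's Tick drains excess above MaxHealth (also used for armor), syncing via server events.
; Authority-only TakeDamage splits hits 80/20 between armor and health.
; Death is checked only without armor, updating kills, deaths and score, penalizing suicides.
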(event EventBeginPlay
  (bind _asbp_player (Utilities|Casting|CastToBP_Player (Components|GetOwner)))
  (Variables|Default|SetPlayer _asbp_player))

(event EventTick
  (params (DeltaSeconds :type Float%20%28single-precision%29))
  (if (Variables|/Game/Game/Player/BP_Player.BP_Player_C|GetIsMine (Variables|Default|GetPlayer))
    (CallFunction|RemoveOverPoints DeltaSeconds)))

(event Custom|ServerSetHealth
  (params (Health :type Float%20%28double-precision%29))
  (Variables|Default|SetHealth Health))

(event Custom|ServerSetArmor
  (params (Armor :type Float%20%28double-precision%29))
  (Variables|Default|SetArmor Armor))

(fn RemoveOverPoints
  (params (DeltaTime :type Float%20%28double-precision%29))
  (Utilities|FlowControl|Sequence
    (:then_0
      (if (> (Variables|Default|GetHealth) (Variables|Default|GetMaxHealth))
        (bind _output_get (Variables|Default|SetHealth (- (Variables|Default|GetHealth) (* (Variables|Default|GetRemovePointsSpeed) DeltaTime))))
        (CallFunction|ServerSetHealth _output_get)))
    (:then_1
      (if (> (Variables|Default|GetArmor) (Variables|Default|GetMaxHealth))
        (bind _output_get_2 (Variables|Default|SetArmor (- (Variables|Default|GetArmor) (* (Variables|Default|GetRemovePointsSpeed) DeltaTime))))
        (CallFunction|ServerSetArmor _output_get_2)))))

(fn AddPoints
  (params (Type :type E_PlayerPoints%20Enum :default "NewEnumerator0") (Points :type Float%20%28double-precision%29) (Buffed :type Boolean))
  (LocalVariables|SetIsBuff Buffed)
  (switch Utilities|FlowControl|Switch|SwitchonE_PlayerPoints Type
    (:NewEnumerator0
      (bind _output_get (CallFunction|CalculatePoints Points (Variables|Default|GetHealth) (Variables|Default|GetMaxHealth) (Variables|Default|GetMaxBuffedHealth) (LocalVariables|GetIsBuff)))
      (bind _output_get_2 (Variables|Default|SetHealth _output_get))
      (CallFunction|ServerSetHealth _output_get_2))
    (:NewEnumerator1
      (bind _output_get_3 (CallFunction|CalculatePoints Points (Variables|Default|GetArmor) (Variables|Default|GetMaxArmor) (Variables|Default|GetMaxBuffedAmor) (LocalVariables|GetIsBuff)))
      (bind _output_get_4 (Variables|Default|SetArmor _output_get_3))
      (CallFunction|ServerSetArmor _output_get_4))))

(fn CalculatePoints
  (params (Points :type Float%20%28double-precision%29) (Value :type Float%20%28double-precision%29) (MaxValue :type Float%20%28double-precision%29) (MaxBufferValue :type Float%20%28double-precision%29) (IsBuff :type Boolean))
  (LocalVariables|SetTagetValue (+ Points Value))
  (if IsBuff
    (bind _output_get (LocalVariables|SetTagetValue (Math|Float|Clamp(Float) (LocalVariables|GetTagetValue) 0.0 MaxBufferValue)))
    (return _output_get)
    (else
      (bind _output_get_2 (LocalVariables|SetTagetValue (Math|Float|Clamp(Float) (LocalVariables|GetTagetValue) 0.0 MaxValue)))
      (return _output_get_2))))

(fn IsCanAdd
  (params (IsBuff :type Boolean) (Type :type E_PlayerPoints%20Enum :default "NewEnumerator0") (Value :type Float%20%28double-precision%29))
  (if IsBuff
    (return true Value)
    (else
      (switch Utilities|FlowControl|Switch|SwitchonE_PlayerPoints Type
        (:NewEnumerator0
          (if (< (Variables|Default|GetHealth) (Variables|Default|GetMaxHealth))
            (return true Value)
            (else
              (return false 0.0))))
        (:NewEnumerator1
          (if (< (Variables|Default|GetArmor) (Variables|Default|GetMaxArmor))
            (if true
              (return true Value))
            (else
              (return false 0.0))))))))

(fn TakeDamage
  (params (Value :type Float%20%28double-precision%29) (DamageType :type E_DamageType%20Enum :default "NewEnumerator0") (Damager :type BP%20Player%20Controller%20Object%20Reference))
  (Networking|SwitchHasAuthority
    (:Authority
      (Variables|Default|SetDamager Damager)
      (if (> (Variables|Default|GetArmor) 0.0)
        (Variables|Default|SetHealth (Math|Float|Clamp(Float) (- (Variables|Default|GetHealth) (* Value 0.2)) 0.0 (Variables|Default|GetMaxBuffedHealth)))
        (Variables|Default|SetArmor (Math|Float|Clamp(Float) (- (Variables|Default|GetArmor) (* Value 0.8)) 0.0 (Variables|Default|GetMaxBuffedAmor)))
        (else
          (bind _output_get (Variables|Default|SetHealth (Math|Float|Clamp(Float) (- (Variables|Default|GetHealth) Value) 0.0 (Variables|Default|GetMaxBuffedHealth))))
          (if (<= _output_get 0.0)
            (bind _asbp_player_controller (Utilities|Casting|CastToBP_PlayerController (Pawn|GetController (Variables|Default|GetPlayer))))
            (LocalVariables|SetCurrentController _asbp_player_controller)
            (Default|OnDead (Variables|Default|GetPlayer))
            (Default|DeadPlayer (LocalVariables|GetCurrentController))
            (if (== (LocalVariables|GetCurrentController) (Variables|Default|GetDamager))
              (Default|AddDeath (LocalVariables|GetCurrentController))
              (Default|AddScore (LocalVariables|GetCurrentController) -1)
              (Default|ApplyStats (LocalVariables|GetCurrentController))
              (else
                (Default|AddScore (Variables|Default|GetDamager) 1)
                (Default|AddKill (Variables|Default|GetDamager))
                (Default|AddDeath (LocalVariables|GetCurrentController))
                (Default|ApplyStats (LocalVariables|GetCurrentController))))))))))