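; Player component that switches between six weapon slots by input, using the shared weapon list and the player's inventory.
; Switches require an owned, different weapon and an idle current one, then wait out the de-equip montage before replacing the weapon's child actor.
; ChangeWeaponServer stores the current ID and calls ChangeWeaponClient, which gives non-local players a third-person mesh, materials and offset transform, plus a child weapon actor with its mesh disabled.
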(event Custom|OnChangeWeapon
  (params (NewID :type Integer) (FindedWeapon :type Weapon%20Class%20Reference))
  (bind _player (Variables|Default|GetPlayer))
  (Variables|Default|SetWaitForDeEquip true)
  (bind _asbp_base_weapon (Utilities|Casting|CastToBP_BaseWeapon (Variables|/Script/Engine.ChildActorComponent|GetChildActor (Variables|Default|GetSpawnedWeapon))))
  (Class|Weapon|DeEquipAnimation _asbp_base_weapon)
  (Utilities|FlowControl|Delay (Animation|GetPlayLength (Variables|/Game/Game/Player/Weapons/BP_BaseWeapon.BP_BaseWeapon_C|GetDeEquip_Montage _asbp_base_weapon)))
  (Variables|Default|SetWaitForDeEquip false)
  (Default|DestroyWeaponChild _player)
  (CallFunction|CreateChildActorWeapon NewID FindedWeapon _player)
  (CallFunction|ChangeWeaponServer NewID))

(event Custom|ChangeWeaponServer
  (params (Value :type Integer))
  (Variables|Default|SetCurrentWeapon Value)
  (CallFunction|ChangeWeaponClient))

(event Custom|ChangeWeaponClient
  (bind _player (Variables|Default|GetPlayer))
  (bind _weaponslist (Variables|Default|GetWeaponsList))
  (bind _currentweapon (Variables|Default|GetCurrentWeapon))
  (bind (_value _returnvalue) (Utilities|Map|Find _weaponslist _currentweapon))
  (bind _clientweapon (Variables|/Game/Game/Player/BP_Player.BP_Player_C|GetClientWeapon _player))
  (if (not (Variables|/Game/Game/Player/BP_Player.BP_Player_C|GetIsMine (Variables|Default|GetPlayer)))
    (if _returnvalue
      (CallFunction|ClientWeaponCreate _value _clientweapon)
      (ChildActorComponent|SetChildActorClass _clientweapon (Variables|/Script/ShooterRooms.WeaponDataAsset|GetweaponClass _value))
      (bind _asbp_base_weapon (Utilities|Casting|CastToBP_BaseWeapon (Variables|/Script/Engine.ChildActorComponent|GetChildActor _clientweapon)))
      (Default|DisableMesh _asbp_base_weapon))))

(event Input|ActionEvents|InputActionWeapon4
  (params (Key :type Key%20Structure))
  (:Pressed
    (CallFunction|SpawnWeapon 4)))

(event Input|ActionEvents|InputActionWeapon5
  (params (Key :type Key%20Structure))
  (:Pressed
    (CallFunction|SpawnWeapon 5)))

(event Input|ActionEvents|InputActionWeapon6
  (params (Key :type Key%20Structure))
  (:Pressed
    (CallFunction|SpawnWeapon 6)))

(event Input|ActionEvents|InputActionWeapon1
  (params (Key :type Key%20Structure))
  (:Pressed
    (CallFunction|SpawnWeapon 1)))

(event Input|ActionEvents|InputActionWeapon2
  (params (Key :type Key%20Structure))
  (:Pressed
    (CallFunction|SpawnWeapon 2)))

(event Input|ActionEvents|InputActionWeapon3
  (params (Key :type Key%20Structure))
  (:Pressed
    (CallFunction|SpawnWeapon 3)))

(fn SpawnWeapon
  (params (ID :type Integer))
  (if (not (Variables|Default|GetWaitForDeEquip))
    (bind _have (Default|GetWeaponbyID (Variables|/Game/Game/Player/BP_Player.BP_Player_C|GetBP_InventoryComponent (Variables|Default|GetPlayer)) ID))
    (if (and (!= ID (Variables|Default|GetCurrentWeapon)) _have)
      (bind _output_get (LocalVariables|SetNewID ID))
      (if (.ReturnValue (Utilities|Map|Find (Variables|Default|GetWeaponsList) _output_get))
        (LocalVariables|SetFindedWeapon (Variables|/Script/ShooterRooms.WeaponDataAsset|GetweaponClass (.Value (Utilities|Map|Find (Variables|Default|GetWeaponsList) _output_get))))
        (Utilities|IsValid (Variables|Default|GetSpawnedWeapon)
          (:Is%20Valid
            (bind _asweapon (Utilities|Casting|CastToWeapon (Variables|/Script/Engine.ChildActorComponent|GetChildActor (Variables|Default|GetSpawnedWeapon))))
            (if (and (Utilities|Enum|Equal(Enum) (Variables|/Script/ShooterRooms.Weapon|GetweaponState _asweapon) "VE_Idle") (== (Variables|/Script/ShooterRooms.Weapon|GetwaitForEquip _asweapon) false))
              (CallFunction|OnChangeWeapon (LocalVariables|GetNewID) (LocalVariables|GetFindedWeapon))))
          (:Is%20Not%20Valid
            (CallFunction|CreateChildActorWeapon (LocalVariables|GetNewID) (LocalVariables|GetFindedWeapon) (Variables|Default|GetPlayer))))))))

(fn GetWeaponbyID
  (params (ID :type Integer))
  (bind _weaponslist (Variables|Default|GetWeaponsList))
  (bind (_value _returnvalue) (Utilities|Map|Find _weaponslist ID))
  (if _returnvalue
    (return _value)
    (else
      (return 0))))

(fn CreateChildActorWeapon
  (params (ID :type Integer) (Weapon :type Actor%20Class%20Reference) (Player :type BP%20Player%20Object%20Reference))
  (bind _returnvalue (Default|AddWeaponChild Player))
  (ChildActorComponent|SetChildActorClass _returnvalue Weapon)
  (Variables|Default|SetCurrentWeapon ID)
  (Variables|Default|SetSpawnedWeapon _returnvalue))

(fn Setup
  (bind _returnvalue (Components|GetOwner))
  (Variables|Default|SetWeaponsList (Variables|/Script/ShooterRooms.WorldData|GetweaponsList (Variables|Default|GetWorldData)))
  (Variables|Default|SetHandle (Class|Actor|FindComponentbyTag _returnvalue "/Script/Engine.ArrowComponent" "Handle"))
  (bind _asbp_player (Utilities|Casting|CastToBP_Player _returnvalue))
  (bind _output_get (Variables|Default|SetPlayer _asbp_player))
  (if (Variables|/Game/Game/Player/BP_Player.BP_Player_C|GetIsMine _output_get)
    (CallFunction|SpawnWeapon 1)
    (CallFunction|ChangeWeaponServer 1)
    (CallFunction|ChangeWeaponClient)
    (else
      (Variables|Default|SetStartWeaponTransform (Transformation|GetRelativeTransform (Variables|/Game/Game/Player/BP_Player.BP_Player_C|GetWeapon _output_get))))))

(fn ChangeMaterials
  (params (Array :type Array%20of%20Material%20Interface%20Object%20References))
  (for (_array_element _array_index) Array
    (Rendering|Material|SetMaterial (Variables|/Game/Game/Player/BP_Player.BP_Player_C|GetWeapon (Variables|Default|GetPlayer)) _array_index _array_element)))

(fn ClientWeaponCreate
  (params (WeaponData :type Weapon%20Data%20Asset%20Object%20Reference) (ChildActor :type Child%20Actor%20Component%20Object%20Reference))
  (bind _startweapontransform (Variables|Default|GetStartWeaponTransform))
  (bind _clienttransformoffcet (Variables|/Script/ShooterRooms.WeaponDataAsset|GetclientTransformOffcet WeaponData))
  (Components|SkeletalMesh|SetSkeletalMeshAsset (Variables|/Game/Game/Player/BP_Player.BP_Player_C|GetWeapon (Variables|Default|GetPlayer)) (Variables|/Script/ShooterRooms.WeaponDataAsset|Getmesh WeaponData))
  (CallFunction|ChangeMaterials (Variables|/Script/ShooterRooms.WeaponDataAsset|GetclientMaterals WeaponData))
  (Transformation|SetRelativeTransform (Variables|/Game/Game/Player/BP_Player.BP_Player_C|GetWeapon (Variables|Default|GetPlayer)) (Math|Transform|MakeTransform (+ (.location _clienttransformoffcet) (.location _startweapontransform)) (Math|Rotator|CombineRotators (.rotation _clienttransformoffcet) (.rotation _startweapontransform)) (+ (.scale _clienttransformoffcet) (.scale _startweapontransform))) false false))