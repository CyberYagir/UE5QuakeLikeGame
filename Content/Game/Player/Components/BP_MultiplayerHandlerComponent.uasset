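; BP_MultiplayerHandlerComponent is a player component that handles the networked side of weapon fire.
; Server events spawn pistol, rocket and grenade projectiles, with grenades launched by physics velocity plus part of the owner's motion.
; Railgun, shotgun and shaft use line traces to apply damage through BPStatsComponent; railgun and shotgun then pass shot data to RPC events for beam or decal effects.
; Shaft state is sent to the server only when firing toggles or its position moves noticeably.
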(event Custom|ShootPistolServer
  (params (Transform :type Transform))
  ;[1 0 0.4688] Pistol Server
  (bind _returnvalue (Game|SpawnActorfromClass "/Game/Game/Player/Weapons/Bullets/BP_ProjectTile.BP_ProjectTile_C" Transform "AlwaysSpawn" "MultiplyWithRoot" (Components|GetOwner) 0))
  (Default|SetPlayer _returnvalue (Components|GetOwner)))

(event Custom|GetPlayer
  ;[0 0.2266 1] Get Player
  (bind _asbp_player (Utilities|Casting|CastToBP_Player (Components|GetOwner)))
  (bind _asbp_player_controller (Utilities|Casting|CastToBP_PlayerController (Pawn|GetController _asbp_player)))
  (Variables|Default|SetAs%20BP%20Player%20Controller _asbp_player_controller))

(event Custom|ShootShaftUpdateServer
  (params (NewShaftData :type ST%20Shaft%20Status%20Structure))
  ;[1 0.3281 0] Shaft
  ;;[1 0.09375 0] Shaft Server
  (Variables|Default|SetShaftData NewShaftData))

(event Custom|ShootShaftUpdate
  (params (NewShaftData :type ST%20Shaft%20Status%20Structure))
  (bind (_isshooted _position) (Utilities|Struct|BreakST_ShaftStatus NewShaftData))
  (bind _shaftdata (Variables|Default|GetShaftData))
  (bind (_isshooted_2 _position_2) (Utilities|Struct|BreakST_ShaftStatus _shaftdata))
  ;[1 0.3281 0] Shaft
  ;;[0.2187 1 0] Shaft Update
  (if (or (!= _isshooted _isshooted_2) (and (> (Math|Vector|VectorLengthSquared (- _position _position_2)) 1.0) _isshooted))
    (CallFunction|ShootShaftUpdateServer NewShaftData)))

(event Custom|ShootRocketServer
  (params (Transform :type Transform))
  ;[0 1 1] Rocket Server
  (bind _returnvalue (Game|SpawnActorfromClass "/Game/Game/Player/Weapons/Bullets/BP_Rocket.BP_Rocket_C" Transform "AlwaysSpawn" "MultiplyWithRoot" (Components|GetOwner) 0))
  (Default|SetPlayer _returnvalue (Components|GetOwner)))

(event Custom|ShootShaftDamageServer
  (params (StartPos :type Vector) (EndPos :type Vector) (Damage :type Float%20%28double-precision%29))
  ;[1 0.3281 0] Shaft
  ;;[0 0.25 1] Shaft RPC
  (bind (_outhit _returnvalue) (Collision|LineTraceForObjects StartPos EndPos (Variables|Default|GetHitTypes) false (Utilities|Array|MakeArray (Components|GetOwner)) "ForDuration"))
  (if _returnvalue
    (bind _asbp_player (Utilities|Casting|CastToBP_Player (.HitActor (Collision|BreakHitResult _outhit))))
    (Default|TakeDamage (Variables|/Game/Game/Player/BP_Player.BP_Player_C|GetBP_StatsComponent _asbp_player) Damage "NewEnumerator0" (Variables|Default|GetAs%20BP%20Player%20Controller))))

(event Custom|ShootGranadeServer
  (params (Transform :type Transform) (ForwardVector :type Vector) (Force :type Float%20%28double-precision%29))
  (bind _returnvalue (Components|GetOwner))
  ;[0.5469 1 0] Granade Server
  (bind _returnvalue_2 (Game|SpawnActorfromClass "/Game/Game/Player/Weapons/Bullets/BP_GranadeBullet.BP_GranadeBullet_C" Transform "AlwaysSpawn" "MultiplyWithRoot" _returnvalue 0))
  (Default|SetPlayer _returnvalue_2 _returnvalue)
  (Transformation|AddActorLocalRotation _returnvalue_2 "90.000000,0.000000,0.000000" false false)
  (Transformation|AddActorLocalRotation _returnvalue_2 (Math|Random|RandomRotator true) false false)
  (Physics|SetPhysicsLinearVelocity (Variables|/Game/Game/Player/Weapons/Bullets/BP_GranadeBullet.BP_GranadeBullet_C|GetGranade _returnvalue_2) (+ (* ForwardVector Force) (* (Transformation|GetVelocity (Components|GetOwner)) 0.3) "0.000000,0.000000,350.000000") true "None"))

(event Custom|ShootRailRPC
  (params (Transform :type Transform) (EndPoint :type Vector) (CameraPoint :type Vector))
  (bind (_location _rotation _scale) (Math|Transform|BreakTransform Transform))
  ;[1 0.2812 0] Railgun
  ;;[1 0.6094 0] Rail RPC
  (bind _asbp_player (Utilities|Casting|CastToBP_Player (Components|GetOwner)))
  (bind _returnvalue (Game|SpawnActorfromClass "/Game/Game/Player/Weapons/Bullets/BP_RailBullet.BP_RailBullet_C" (Math|Transform|MakeTransform (Transformation|GetSocketLocation (Variables|/Game/Game/Player/BP_Player.BP_Player_C|GetWeapon _asbp_player) "ShootPoint") _rotation _scale) "AlwaysSpawn" "MultiplyWithRoot" (Components|GetOwner) 0))
  (bind (_outhit _returnvalue_2) (Collision|LineTraceForObjects CameraPoint EndPoint (Variables|Default|GetHitTypes) false 0 "None"))
  (if _returnvalue_2
    (CallFunction|SpawnDecal (.hitcomponent _outhit) (.impactpoint _outhit) (Math|Rotator|MakeRotfromX (.normal _outhit)) 4.0 "/Game/Game/Player/Data/Decals/DA_HoleDecal.DA_HoleDecal")
    (Default|Init _returnvalue (.impactpoint _outhit))
    (else
      (Default|Init _returnvalue EndPoint))))

(event Custom|ShootRailServer
  (params (Transform :type Transform) (EndPoint :type Vector) (CameraPoint :type Vector) (Damage :type Float%20%28double-precision%29))
  ;[1 0.2812 0] Railgun
  ;;[0.7109 1 0] Rail Server
  (bind (_outhit _returnvalue) (Collision|LineTraceForObjects CameraPoint EndPoint (Variables|Default|GetHitTypes) false 0 "None"))
  (if _returnvalue
    (bind _asbp_player (Utilities|Casting|CastToBP_Player (.HitActor (Collision|BreakHitResult _outhit)))
      (:then
        (Default|TakeDamage (Variables|/Game/Game/Player/BP_Player.BP_Player_C|GetBP_StatsComponent _asbp_player) Damage "NewEnumerator6" (Variables|Default|GetAs%20BP%20Player%20Controller)))
      (:CastFailed
        _)))
  (CallFunction|ShootRailRPC Transform EndPoint CameraPoint))

(event Custom|ShootShotgunRPC
  (params (Bursts :type Array%20of%20ST%20Burst%20Structures))
  ;[1 0.75 0] Shotgun
  ;;[1 0 0.2812] RPC Shotgun
  (for _array_element Bursts
    (CallFunction|SpawnDecal (.component _array_element) (.location _array_element) (.rotation _array_element) 5.0 "/Game/Game/Player/Data/Decals/DA_HoleDecal.DA_HoleDecal")))

(event Custom|ShootShotgunServer
  (params (CameraRotation :type Rotator) (CameraLocation :type Vector) (BurstCount :type Integer) (Spread :type Float%20%28double-precision%29) (Damage :type Float%20%28double-precision%29))
  ;[1 0.75 0] Shotgun
  ;;[1 0 0.6328] Server Shotgun
  (Utilities|Array|Clear (Variables|Default|GetBurstsTmpList))
  (for _index (range 0 BurstCount)
    (bind _returnvalue (CallFunction|CreateRandomRotator Spread))
    (bind (_outhit _returnvalue_2) (Collision|LineTraceForObjects CameraLocation (+ CameraLocation (* (Math|Vector|GetForwardVector (Math|Rotator|CombineRotators CameraRotation _returnvalue)) 10000)) (Variables|Default|GetHitTypes) false 0 "None"))
    (if _returnvalue_2
      (bind _asbp_player (Utilities|Casting|CastToBP_Player (.HitActor (Collision|BreakHitResult _outhit)))
        (:then
          (Default|TakeDamage (Variables|/Game/Game/Player/BP_Player.BP_Player_C|GetBP_StatsComponent _asbp_player) Damage "NewEnumerator2" (Variables|Default|GetAs%20BP%20Player%20Controller)))
        (:CastFailed
          _))
      (Game|SpawnActorfromClass "/Game/Game/Player/Weapons/Bullets/BP_Burst.BP_Burst_C" (Math|Transform|MakeTransform (.Location (Collision|BreakHitResult _outhit)) (Math|Conversions|RotationFromXVector (.Normal (Collision|BreakHitResult _outhit))) "1.000000,1.000000,1.000000") "AlwaysSpawn" "MultiplyWithRoot" (Components|GetOwner) 0)
      (Utilities|Array|Add (Variables|Default|GetBurstsTmpList) (Utilities|Struct|MakeST_Burst (.HitComponent (Collision|BreakHitResult _outhit)) (.Location (Collision|BreakHitResult _outhit)) (Math|Conversions|RotationFromXVector (.Normal (Collision|BreakHitResult _outhit)))))))
  (CallFunction|ShootShotgunRPC (Variables|Default|GetBurstsTmpList)))

(event EventBeginPlay
  (CallFunction|GetPlayer))