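; Player inventory component that stores owned weapons and their ammo as an item array keyed by weapon ID.
; AddWeapon appends new weapons or refills owned ones, raising low ammo to a minimum or topping up toward a maximum, using limits from the player's weapon switch component.
; It answers lookup and can-shoot queries, while RemoveBullet drains ammo per shot or scaled by delta time.
; Startup and inventory changes fire a change event.
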(event EventBeginPlay
  (bind _asbp_player (Utilities|Casting|CastToBP_Player (Components|GetOwner)))
  (bind _output_get (Variables|Default|SetPlayer _asbp_player))
  (Variables|Default|SetWeaponSwitch (Variables|/Game/Game/Player/BP_Player.BP_Player_C|GetBP_WeaponSwichComponent _output_get))
  (Default|CallChangeInventoryEvent))

(fn AddWeapon
  (params (Item :type ST%20Item%20Structure))
  (bind (_array_element _array_index) (Utilities|Array|ForEachLoopwithBreak (Variables|Default|GetWeapons))
    (:LoopBody
      (LocalVariables|SetFindedIndex _array_index)
      (LocalVariables|SetFindedBulletsCount (.Bullets (Utilities|Struct|BreakST_Item _array_element)))
      (if (== (.WeaponID (Utilities|Struct|BreakST_Item _array_element)) (.WeaponID (Utilities|Struct|BreakST_Item Item)))
        (bind _value (Default|GetWeaponbyID (Variables|Default|GetWeaponSwitch) (.WeaponID (Utilities|Struct|BreakST_Item Item))))
        (LocalVariables|SetFindedRef (Utilities|Array|Get(acopy) (Variables|Default|GetWeapons) (LocalVariables|GetFindedIndex)))
        (if (<= (Variables|/Script/ShooterRooms.WeaponDataAsset|GetminBullets _value) (Class|KismetMathLibrary|ToInt64(Float) (LocalVariables|GetFindedBulletsCount)))
          (if (< (LocalVariables|GetFindedBulletsCount) (Variables|/Script/ShooterRooms.WeaponDataAsset|GetmaxBullets _value))
            (bind _structout (Utilities|Struct|SetmembersinST_Item (LocalVariables|GetFindedRef) (Math|Conversions|ToFloat(Integer) (Math|Integer|Clamp(Integer) (+ (.Bullets (Utilities|Struct|BreakST_Item (LocalVariables|GetFindedRef))) (Variables|/Script/ShooterRooms.WeaponDataAsset|GetsecondaryAddAmmoValue _value)) 0 (Variables|/Script/ShooterRooms.WeaponDataAsset|GetmaxBullets _value)))))
            (Utilities|Array|SetArrayElem (Variables|Default|GetWeapons) (LocalVariables|GetFindedIndex) _structout)
            (Default|CallChangeInventoryEvent)
            (return _structout true)
            (else
              (return (LocalVariables|GetFindedRef) false)))
          (else
            (bind _structout_2 (Utilities|Struct|SetmembersinST_Item (LocalVariables|GetFindedRef) (Math|Conversions|ToFloat(Integer) (Variables|/Script/ShooterRooms.WeaponDataAsset|GetminBullets _value))))
            (Utilities|Array|SetArrayElem (Variables|Default|GetWeapons) (LocalVariables|GetFindedIndex) _structout_2)
            (Default|CallChangeInventoryEvent)
            (return _structout_2 true)))))
    (:Completed
      (bind _returnvalue (Utilities|Array|Add (Variables|Default|GetWeapons) Item))
      (Default|CallChangeInventoryEvent)
      (return (Utilities|Array|Get(acopy) (Variables|Default|GetWeapons) _returnvalue) false))))

(fn IsCanShoot
  (params (ID :type Integer))
  (for _array_element (Variables|Default|GetWeapons)
    (if (== (.WeaponID (Utilities|Struct|BreakST_Item _array_element)) ID)
      (if (> (.Bullets (Utilities|Struct|BreakST_Item _array_element)) 0.0)
        (return true))))
  (return false))

(fn GetWeaponbyID
  (params (Index :type Integer))
  (for _array_element (Variables|Default|GetWeapons)
    (if (== (.WeaponID (Utilities|Struct|BreakST_Item _array_element)) Index)
      (return _array_element true)))
  (return (Utilities|Struct|MakeST_Item -1 -1.0) false))

(fn RemoveBullet
  (params (Index :type Integer) (UseDeltaTime :type Boolean))
  (LocalVariables|SetIsUseDelta UseDeltaTime)
  (LocalVariables|SetWeaponIndex Index)
  (bind (_array_element _array_index) (Utilities|Array|ForEachLoopwithBreak (Variables|Default|GetWeapons))
    (:LoopBody
      (LocalVariables|SetLoopIndex _array_index)
      (LocalVariables|SetCurrentWeaponID (.WeaponID (Utilities|Struct|BreakST_Item _array_element)))
      (LocalVariables|SetCurrentBulletsCount (.Bullets (Utilities|Struct|BreakST_Item _array_element)))
      (if (== (LocalVariables|GetCurrentWeaponID) (LocalVariables|GetWeaponIndex))
        (bind _value (Default|GetWeaponbyID (Variables|Default|GetWeaponSwitch) (LocalVariables|GetCurrentWeaponID)))
        (LocalVariables|SetCurrentWeaponClass _value)
        (if (LocalVariables|GetIsUseDelta)
          (LocalVariables|SetDeltaTime (Utilities|Time|GetWorldDeltaSeconds))
          (else
            (LocalVariables|SetDeltaTime 1.0)))
        (Utilities|Struct|SetmembersinST_Item (Utilities|Array|Get(acopy) (Variables|Default|GetWeapons) (LocalVariables|GetLoopIndex)) (Math|Float|Clamp(Float) (- (LocalVariables|GetCurrentBulletsCount) (* (Variables|/Script/ShooterRooms.WeaponDataAsset|GetremoveBullets (LocalVariables|GetCurrentWeaponClass)) (LocalVariables|GetDeltaTime))) 0.0 999.0))
        (Default|CallChangeInventoryEvent)))))