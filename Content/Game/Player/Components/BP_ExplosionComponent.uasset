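; BP_ExplosionComponent is an actor component that deals explosion damage to players within a radius.
; DamagePlayer centers on the owner's location, or on the stored position when CustomPosition is set, and sphere-overlaps for BP_Player pawns.
; It traces the Camera channel toward each capsule and damages any player hit through BPStatsComponent, scaling Damage by a distance-based curve.
; Debug sphere, trace drawing and damage printing remain active.
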(fn DamagePlayer
  (params (Sender :type BP%20Player%20Controller%20Object%20Reference))
  (LocalVariables|SetSnd Sender)
  (if (Variables|Default|GetCustomPosition)
    _
    (else
      (Variables|Default|SetPos (Transformation|GetActorLocation (Components|GetOwner)))))
  (Rendering|Debug|DrawDebugSphere (Variables|Default|GetPos) (Variables|Default|GetRadius) 12 "(R=1.000000,G=1.000000,B=1.000000,A=1.000000)" 5.0 1.0)
  (bind _outactors (Collision|SphereOverlapActors (Variables|Default|GetPos) (Variables|Default|GetRadius) (Utilities|Array|MakeArray "ObjectTypeQuery3") "/Game/Game/Player/BP_Player.BP_Player_C"))
  (for _array_element _outactors
    (bind _asbp_player (Utilities|Casting|CastToBP_Player _array_element))
    (bind (_outhit _returnvalue) (Collision|LineTraceByChannel (Variables|Default|GetPos) (+ (Variables|Default|GetPos) (* (- (Transformation|GetWorldLocation (Variables|/Script/Engine.Character|GetCapsuleComponent _asbp_player)) (Variables|Default|GetPos)) (Variables|Default|GetRadius))) "TraceTypeQuery2" false 0 "ForDuration"))
    (if _returnvalue
      (bind _asbp_player_2 (Utilities|Casting|CastToBP_Player (.hitactor _outhit)))
      (Development|PrintString (Utilities|String|ToString(Float) (* (Math|Curves|GetFloatValue (Variables|Default|GetDamageCurve) (Math|Float|Clamp(Float) (/ (.distance _outhit) (Variables|Default|GetRadius)))) (Variables|Default|GetDamage))))
      (Default|TakeDamage (Variables|/Game/Game/Player/BP_Player.BP_Player_C|GetBP_StatsComponent _asbp_player_2) (* (Math|Curves|GetFloatValue (Variables|Default|GetDamageCurve) (Math|Float|Clamp(Float) (/ (.distance _outhit) (Variables|Default|GetRadius)))) (Variables|Default|GetDamage)) "NewEnumerator0" (LocalVariables|GetSnd)))))

(fn SetPos
  (params (Vector :type Vector))
  (Variables|Default|SetPos Vector))