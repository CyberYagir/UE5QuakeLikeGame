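; Player component that computes foot IK and hip offsets from the ground height under each foot.
; BeginPlay caches the owning BP_Player's mesh, and UpdateFootIK traces down from actor height at a socket's XY, with debug drawing.
; Update stores each hit's height relative to the mesh and lowers the hips by half the height difference between feet.
; A separate helper samples MoveCurve at a given time.
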(event EventBeginPlay
  (bind _asbp_player (Utilities|Casting|CastToBP_Player (Components|GetOwner)))
  (bind _output_get (Variables|Default|SetAs%20BP%20Player _asbp_player))
  (Variables|Default|SetMesh (Variables|/Script/Engine.Character|GetMesh _output_get)))

(fn UpdateFootIK
  (params (Socket :type Name))
  (bind _returnvalue (Components|GetOwner))
  (bind _mesh (Variables|Default|GetMesh))
  (bind _returnvalue_2 (Transformation|GetSocketLocation _mesh Socket))
  (bind _returnvalue_3 (Transformation|GetActorLocation _returnvalue))
  (bind (_x _y) (Math|Vector|BreakVector _returnvalue_2))
  (bind _z (Math|Vector|BreakVector _returnvalue_3))
  (bind _returnvalue_4 (Math|Vector|MakeVector _x _y _z))
  (bind (_outhit _returnvalue_5) (Collision|LineTraceByChannel _returnvalue_4 (+ _returnvalue_4 (Math|Vector|MakeVector 0.0 0.0 -5e+02)) "TraceTypeQuery1" false 0 "ForDuration"))
  (if _returnvalue_5
    (return (.location _outhit) (.z (- (.location _outhit) (Transformation|GetWorldLocation (Variables|Default|GetMesh)))))
    (else
      (return "0, 0, 0" 0.0))))

(fn Update
  (bind (_out_hit_location _offcet) (CallFunction|UpdateFootIK (Variables|Default|GetLeftSocket)))
  (Variables|Default|SetLeftOffcet _offcet)
  (bind (_out_hit_location_2 _offcet_2) (CallFunction|UpdateFootIK (Variables|Default|GetRightSocket)))
  (Variables|Default|SetRightOffcet _offcet_2)
  (Variables|Default|SetHipOffcet (* (Math|Float|Absolute(Float) (.z (- _out_hit_location_2 _out_hit_location))) -0.5)))

(fn GetRunCurveValue
  (params (Time :type Float%20%28double-precision%29))
  (return (Math|Curves|GetFloatValue (Variables|Default|GetMoveCurve) Time)))