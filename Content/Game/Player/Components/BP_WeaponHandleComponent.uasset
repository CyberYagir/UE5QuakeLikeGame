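; BP_WeaponHandleComponent is a player component that adds procedural weapon sway by animating the owner's ArrowComponent tagged "Handle".
; BeginPlay caches the handle's rest transform and the owning BP_Player, then Update takes delta time and X/Y input.
; RotateWeapon eases toward the rest rotation offset by scaled input.
; MoveWeapon eases toward the rest position, offset opposite the player's local movement direction, independent of speed magnitude.
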(event EventBeginPlay
  (bind _output_get (Variables|Default|SetHandle (Class|Actor|FindComponentbyTag (Components|GetOwner) "/Script/Engine.ArrowComponent" "Handle")))
  (Variables|Default|SetStartRotation (Variables|/Script/Engine.SceneComponent|GetRelativeRotation _output_get))
  (Variables|Default|SetStartPos (Variables|/Script/Engine.SceneComponent|GetRelativeLocation _output_get))
  (bind _asbp_player (Utilities|Casting|CastToBP_Player (Components|GetOwner)))
  (Variables|Default|SetPlayer _asbp_player))

(fn Update
  (params (Delta :type Float%20%28double-precision%29) (X :type Float%20%28double-precision%29) (Y :type Float%20%28double-precision%29))
  (Variables|Default|SetDelta Delta)
  (CallFunction|RotateWeapon X Y)
  (CallFunction|MoveWeapon))

(fn RotateWeapon
  (params (Pitch :type Float%20%28single-precision%29) (Yaw :type Float%20%28single-precision%29))
  (bind _output_get (Variables|Default|SetTargetRotation (Math|Rotator|CombineRotators (Variables|Default|GetStartRotation) (* (Math|Rotator|MakeRotator 0.0 Yaw Pitch) (Variables|Default|GetStrength)))))
  (Transformation|SetRelativeRotation (Variables|Default|GetHandle) (Math|Rotator|Lerp(Rotator) (Variables|/Script/Engine.SceneComponent|GetRelativeRotation (Variables|Default|GetHandle)) _output_get (* (Variables|Default|GetDelta) (Variables|Default|GetBackStrength)) true) false false))

(fn MoveWeapon
  (Transformation|SetRelativeLocation (Variables|Default|GetHandle) (Math|Vector|Lerp(Vector) (Variables|/Script/Engine.SceneComponent|GetRelativeLocation (Variables|Default|GetHandle)) (+ (Variables|Default|GetStartPos) (* (Math|Transform|InverseTransformDirection (Transformation|GetActorTransform (Variables|Default|GetPlayer)) (Math|Vector|Normalize (Variables|/Script/Engine.MovementComponent|GetVelocity (Variables|/Script/Engine.Character|GetCharacterMovement (Variables|Default|GetPlayer))))) (Variables|Default|GetMoveOffcet) -1.0)) (* (Variables|Default|GetDelta) (Variables|Default|GetMoveSpeed))) false false))