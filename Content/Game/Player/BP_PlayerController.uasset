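; Player controller for a match-based game, handling spawning, spectating, death and score UI.
; On local BeginPlay it checks game state, then either spawns a spectator with a random name or moves to the end-game preview camera.
; Spawn, name and stat events forward to BP_GameMode.
; Death unpossesses the pawn, spawns a spectator at its camera and destroys the body after a delay, while holding Tab shows scores.
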(event Custom|SetPlayerName
  (params (Name :type Name))
  (bind _output_get (Variables|Default|SetPlayerName Name))
  (bind _asbp_game_mode (Utilities|Casting|CastToBP_GameMode (Game|GetGameMode)))
  (Default|SetPlayerName _asbp_game_mode self _output_get))

(event Custom|Spawn_Player
  (bind _asbp_game_mode (Utilities|Casting|CastToBP_GameMode (Game|GetGameMode)))
  (Default|SpawnPlayer _asbp_game_mode self))

(event Custom|AddKill
  (bind _asbp_game_mode (Utilities|Casting|CastToBP_GameMode (Game|GetGameMode)))
  (Default|AddKill _asbp_game_mode self))

(event Custom|SetEndPreview
  (bind _outactors (Actor|GetAllActorsOfClass "/Game/Game/Level/BP_EndGameSpawn.BP_EndGameSpawn_C"))
  (bind _asend_game_preview (Utilities|Casting|CastToEndGame_Preview (Variables|/Script/Engine.ChildActorComponent|GetChildActor (Variables|/Game/Game/Level/BP_EndGameSpawn.BP_EndGameSpawn_C|GetChildActor (Utilities|Array|Get(acopy) _outactors)))))
  (bind _asbp_game_mode (Utilities|Casting|CastToBP_GameMode (Game|GetGameMode)))
  (Default|SpawnEndGameController _asbp_game_mode self (Transformation|GetWorldTransform (Variables|/Game/Game/Level/EndGame_Preview.EndGame_Preview_C|GetCamera _asend_game_preview))))

(event Custom|Spawn_Spectrator_OnPos
  (params (Transform :type Transform))
  (bind _self self)
  (bind _asbp_game_mode (Utilities|Casting|CastToBP_GameMode (Game|GetGameMode)))
  (Default|SpawnSpetratoronPose _asbp_game_mode _self Transform)
  (bind _asbp_player_state (Utilities|Casting|CastToBP_PlayerState (Variables|/Script/Engine.Controller|GetPlayerState _self)))
  (Default|ResetTIme _asbp_player_state))

(event Custom|Dead_Player
  (bind _self self)
  (bind _output_get (Variables|Default|SetOldPawn (Pawn|GetControlledPawn _self)))
  (Pawn|UnPossess _self)
  (bind _asbp_player (Utilities|Casting|CastToBP_Player _output_get))
  (CallFunction|SpawnSpectratoronPos (Transformation|GetWorldTransform (Variables|/Game/Game/Player/BP_Player.BP_Player_C|GetCamera _asbp_player)))
  (Utilities|FlowControl|Delay 5.0)
  (Actor|DestroyActor (Variables|Default|GetOldPawn)))

(event Custom|ApplyStats
  (bind _asbp_game_mode (Utilities|Casting|CastToBP_GameMode (Game|GetGameMode)))
  (Default|ApplyScores _asbp_game_mode))

(event Custom|AddDeath
  (bind _asbp_game_mode (Utilities|Casting|CastToBP_GameMode (Game|GetGameMode)))
  (Default|AddDeath _asbp_game_mode self))

(event Custom|Spawn_Spectrator
  (bind _asbp_game_mode (Utilities|Casting|CastToBP_GameMode (Game|GetGameMode)))
  (Default|SpawnSpectrator _asbp_game_mode self))

(event Custom|AddScore
  (params (val :type Integer))
  (bind _asbp_game_mode (Utilities|Casting|CastToBP_GameMode (Game|GetGameMode)))
  (Default|AddScore _asbp_game_mode self val))

(event Custom|DisableUI
  (bind _ui_baseui (Variables|Default|GetUI_BaseUI)
    (:then
      (Variables|/Script/UMG.Widget|SetVisibility _ui_baseui "Hidden"))
    (:else
      _))
  (bind _ui_timer (Variables|Default|GetUI_Timer)
    (:then
      (Variables|/Script/UMG.Widget|SetVisibility _ui_timer "Hidden")
      (bind _ui_respawn (Variables|Default|GetUI_Respawn)
        (:then
          (Variables|/Script/UMG.Widget|SetVisibility _ui_respawn "Hidden"))
        (:else)))
    (:else)))

(event EventBeginPlay
  (if (Pawn|IsLocalPlayerController)
    (bind _asbp_game_state_base (Utilities|Casting|CastToBP_GameStateBase (Game|GetGameState)))
    (if (Utilities|Enum|Equal(Enum) (Variables|/Game/Game/Player/BP_GameStateBase.BP_GameStateBase_C|GetGameState _asbp_game_state_base) "NewEnumerator0")
      (CallFunction|SpawnSpectrator)
      (bind _output_get (Variables|Default|SetPlayerName (Utilities|String|StringToName (Utilities|String|Append "Player" (Utilities|String|ToString(Integer) (Math|Random|RandomInteger 128))))))
      (CallFunction|SetPlayerName _output_get)
      (else
        (CallFunction|SetEndPreview)))))

(event Input|ActionEvents|InputActionTab
  (params (Key :type Key%20Structure))
  (bind _ui_scores (Variables|Default|GetUI_Scores))
  (:Pressed
    (Variables|/Script/UMG.Widget|SetVisibility _ui_scores "Visible"))
  (:Released
    (Variables|/Script/UMG.Widget|SetVisibility _ui_scores "Hidden")))

(fn ConstructionScript)